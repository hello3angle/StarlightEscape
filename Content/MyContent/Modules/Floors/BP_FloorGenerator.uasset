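; BP_FloorGenerator spawns a randomly typed floor piece on BeginPlay, picking Normal, Empty or Breaking and printing the choice for debugging.
; Breaking spawns a BP_BaseDynamicrFloor, Empty spawns a BP_BaseStaticFloor, and Normal spawns a floor with no class shown.
; Each spawn saves the new floor's Arrow world transform as the next SpawnTransform, allowing end-to-end chaining, though GenerateFloors runs only once here.
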(event `self.ReceiveBeginPlay`
  (`self.GenerateFloors`))

(event `self.GenerateFloors`
  (bind _spawn_transform (`self.Spawn Transform`))
  ;[0.2652 1 0.2584] Generator
  (bind _output_get (set `self.FloorType` (cast `/Game/MyContent/Modules/Floors/E_FloorType` (`KismetMathLibrary.Conv_IntToByte` (`KismetMathLibrary.RandomIntegerInRange` 0 2)))))
  ;;[1 0 0.04544] Debug
  (`KismetSystemLibrary.PrintString` (`KismetStringLibrary.Concat_StrStr` "Type: " (`|GetEnumeratorNameAsString` _output_get)) true true (struct :`R` 1.0 :`B` 0.045438 :`A` 1.0))
  (switch `/Game/MyContent/Modules/Floors/E_FloorType` _output_get
    (:`NewEnumerator0`
      (bind _returnvalue (`|SpawnActorFromClass` "/Game/MyContent/Modules/Floors/BP_BaseStaticFloor.BP_BaseStaticFloor_C" _spawn_transform "AlwaysSpawn" "OverrideRootScale" null null))
      (set `self.Spawn Transform` (`SceneComponent.K2_GetComponentToWorld` (`/Game/MyContent/Modules/Floors/BP_BaseStaticFloor.Arrow` _returnvalue))))
    (:`NewEnumerator1`
      (bind _returnvalue_2 (`|SpawnActorFromClass` "/Game/MyContent/Modules/Floors/BP_BaseStaticFloor.BP_BaseStaticFloor_C" _spawn_transform "AlwaysSpawn" "OverrideRootScale" null null))
      (set `self.Spawn Transform` (`SceneComponent.K2_GetComponentToWorld` (`/Game/MyContent/Modules/Floors/BP_BaseStaticFloor.Arrow` _returnvalue_2))))
    (:`NewEnumerator2`
      (bind _returnvalue_3 (`|SpawnActorFromClass` "/Game/MyContent/Modules/Floors/BP_BaseDynamicrFloor.BP_BaseDynamicrFloor_C" _spawn_transform "AlwaysSpawn" "OverrideRootScale" null null))
      (set `self.Spawn Transform` (`SceneComponent.K2_GetComponentToWorld` (`/Game/MyContent/Modules/Floors/BP_BaseDynamicrFloor.Arrow` _returnvalue_3))))))

(fn `UserConstructionScript`)