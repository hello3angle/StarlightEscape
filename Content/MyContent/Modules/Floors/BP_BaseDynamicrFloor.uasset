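; Procedural floor segment that requests the next segment when the player reaches it and removes itself afterward.
; The construction script lays out a random number of five-tile rows of BP_UnitBreakingFloor child actors, then positions a trigger box and arrow by row count.
; The player's first overlap calls the game mode's actor generator to generate floors, and the first exit destroys the segment after a short delay.
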(event `self.Box.OnComponentBeginOverlap`
  (params (OverlappedComponent :type "PrimitiveComponent Object Reference") (OtherActor :type "Actor Object Reference") (OtherComp :type "PrimitiveComponent Object Reference") (OtherBodyIndex :type Integer) (bFromSweep :type Boolean) (SweepResult :type "HitResult Structure (by ref)"))
  (cast `/Game/MyContent/Player/BP_PlayerBase` OtherActor)
  (`/Engine/EditorBlueprintResources/StandardMacros.DoOnce` false
    (:`Completed`
      (bind _asbp_game_mode_base_child (cast `/Game/MyContent/Player/BP_GameModeBase_Child` (`GameplayStatics.GetGameMode`)))
      (message `/Game/MyContent/Modules/Floors/BI_Generator.GenerateFloors` (`/Game/MyContent/Player/BP_GameModeBase_Child.ActorGeneratorRef` _asbp_game_mode_base_child)))))

(event `self.Box.OnComponentEndOverlap`
  (params (OverlappedComponent :type "PrimitiveComponent Object Reference") (OtherActor :type "Actor Object Reference") (OtherComp :type "PrimitiveComponent Object Reference") (OtherBodyIndex :type Integer))
  (cast `/Game/MyContent/Player/BP_PlayerBase` OtherActor)
  (`/Engine/EditorBlueprintResources/StandardMacros.DoOnce` false
    (:`Completed`
      (`KismetSystemLibrary.Delay` 0.5)
      (`self.K2_DestroyActor`))))

(fn `UserConstructionScript`
  (bind (_returnvalue_x _returnvalue_y _returnvalue_z) (`KismetMathLibrary.BreakVector` (`self.K2_GetActorLocation`)))
  (bind _unitsize (`self.UnitSize`))
  (bind (_returnvalue_x_2 _returnvalue_y_2) (`KismetMathLibrary.BreakVector` (- (`self.K2_GetActorLocation`) (`self.SpawnLocation`))))
  (set `self.ScaleX` 2.0)
  (set `self.ScaleY` 2.0)
  (set `self.ScaleZ` 2.0)
  (set `self.SpawnLocation` (`self.K2_GetActorLocation`))
  (bind _output_get (set `self.RowsSpawning` (`KismetMathLibrary.RandomIntegerInRange` 4 (`self.MaxRowsSpawning`))))
  (for _index (range 1 (+ (* _output_get 5) 1))
    (`|ExecutionSequence`
      (:`then_0`
        ;[1 1 1] Add UnitFloorActor
        (bind _returnvalue (`AddComponent|NODE_AddChildActorComponent-1` :`RelativeTransform` (`KismetMathLibrary.MakeTransform` (- (`self.SpawnLocation`) (`KismetMathLibrary.MakeVector` _returnvalue_x (- _returnvalue_y -500.0) _returnvalue_z)))))
        (`ChildActorComponent.SetChildActorClass` _returnvalue "/Game/MyContent/Modules/Floors/BP_UnitBreakingFloor.BP_UnitBreakingFloor_C"))
      (:`then_1`
        ;[1 1 1] Place BoxCollision to Spawn the Next Floor
        (`BoxComponent.SetBoxExtent` (`self.Box`) (`KismetMathLibrary.MakeVector` (* _unitsize 2.0) (* (`self.RowsSpawning`) (`self.ScaleY`) _unitsize) 2000.0) true)
        (`SceneComponent.K2_SetRelativeLocation` (`self.Box`) (`KismetMathLibrary.MakeVector` (* (`self.RowsSpawning`) (`self.ScaleX`) (`self.UnitSize`))) false false))
      (:`then_2`
        ;[1 1 1] Place Arrow to Spawn the Next Floor
        (`SceneComponent.K2_SetRelativeLocation` (`self.Arrow`) (`KismetMathLibrary.MakeVector` (* (`self.RowsSpawning`) (`self.ScaleX`) (`self.UnitSize`))) false false))
      (:`then_3`
        ;[0.2652 1 0.2584] Set to the Next Spawn Location
        (if (== (mod _index 5) 0)
          (set `self.SpawnLocation` (+ (`self.SpawnLocation`) (`KismetMathLibrary.MakeVector` 200.0 _returnvalue_y_2)))
          (else
            (set `self.SpawnLocation` (+ (`self.SpawnLocation`) (0.0 200.0 0.0)))))))))