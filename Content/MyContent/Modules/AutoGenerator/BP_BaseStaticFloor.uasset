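; Base floor segment for an auto-generator, sized at construction from a random row count that sets its X scale.
; The construction script also positions the floor and places a trigger box and arrow along X according to that length, logging the row count.
; When the player leaves the box, the segment destroys itself after a short delay.
; Overlap entry triggers nothing, and the game mode call to generate floors is disconnected.
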(event `self.ReceiveBeginPlay`)

(event `self.Box.OnComponentBeginOverlap`
  (params (OverlappedComponent :type "PrimitiveComponent Object Reference") (OtherActor :type "Actor Object Reference") (OtherComp :type "PrimitiveComponent Object Reference") (OtherBodyIndex :type Integer) (bFromSweep :type Boolean) (SweepResult :type "HitResult Structure (by ref)"))
  (cast `/Game/MyContent/Player/BP_PlayerBase` OtherActor)
  (`/Engine/EditorBlueprintResources/StandardMacros.DoOnce` false))

(event `self.Box.OnComponentEndOverlap`
  (params (OverlappedComponent :type "PrimitiveComponent Object Reference") (OtherActor :type "Actor Object Reference") (OtherComp :type "PrimitiveComponent Object Reference") (OtherBodyIndex :type Integer))
  (cast `/Game/MyContent/Player/BP_PlayerBase` OtherActor)
  (`/Engine/EditorBlueprintResources/StandardMacros.DoOnce` false
    (:`Completed`
      (`KismetSystemLibrary.Delay` 0.5)
      (`self.K2_DestroyActor`))))

(fn `UserConstructionScript`
  (bind _unitsize (`self.UnitSize`))
  (bind _scaley (`self.ScaleY`))
  (bind _output_get (set `self.RowsSpawning` (`KismetMathLibrary.RandomIntegerInRange` 3 (`self.MaxRowsSpawning`))))
  ;[1 0 0.04544] Debug
  (`KismetSystemLibrary.PrintString` (`KismetStringLibrary.Concat_StrStr` "Created " (`KismetStringLibrary.Conv_IntToString` _output_get) " rows") true true (struct :`R` 1.0 :`B` 0.045438 :`A` 1.0))
  (bind _output_get_2 (set `self.ScaleX` (`KismetMathLibrary.Conv_IntToDouble` (* _output_get 2))))
  (`SceneComponent.SetRelativeScale3D` (`self.BaseFloor`) (`KismetMathLibrary.MakeVector` _output_get_2 _scaley (`self.ScaleZ`)))
  (`SceneComponent.K2_SetRelativeLocation` (`self.BaseFloor`) (`KismetMathLibrary.MakeVector` 0.0 (* _scaley (`self.UnitSize`) -0.5)) false false)
  (`BoxComponent.SetBoxExtent` (`self.Box`) (`KismetMathLibrary.MakeVector` (* _unitsize 10.0) (* (`self.ScaleY`) _unitsize) 2000.0) true)
  (`SceneComponent.K2_SetRelativeLocation` (`self.Box`) (`KismetMathLibrary.MakeVector` (* (`self.ScaleX`) (`self.UnitSize`))) false false)
  (`SceneComponent.K2_SetRelativeLocation` (`self.Arrow`) (`KismetMathLibrary.MakeVector` (* (`self.ScaleX`) (`self.UnitSize`))) false false))