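; Breaking floor unit that disappears after a player steps on it and returns after a respawn delay.
; Overlap with BP_PlayerBase runs the StandOn timeline at a StandTime play rate, ramping the material's emissive as warning, then turns the floor off.
; The OnOff timeline animates appearance in both directions while collision toggles on floor and trigger.
; Its Finished pin re-enables the floor after RespawnTime only if off.
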(event `TurnOff`
  (`PrimitiveComponent.SetCollisionEnabled` (`self.BaseFloor`) "NoCollision")
  (`PrimitiveComponent.SetCollisionEnabled` (`self.Trigger`) "NoCollision")
  (set `self.IsOn?` false)
  (bind (_direction _alpha) (`Timeline|On/Off` :!via `ReverseFromEnd` :!label _label)
    (:`Update`
      (`MaterialInstanceDynamic.SetScalarParameterValue` (`self.Material`) "Appearence" _alpha))
    (:`Finished`
      (`KismetSystemLibrary.Delay` (`self.RespawnTime`))
      (if (not (`self.IsOn?`))
        (`self.TurnOn`)))))

(event `TurnOn`
  (`MaterialInstanceDynamic.SetScalarParameterValue` (`self.Material`) "Emissive" 0.0)
  (`PrimitiveComponent.SetCollisionEnabled` (`self.BaseFloor`) "QueryOnly")
  (`PrimitiveComponent.SetCollisionEnabled` (`self.Trigger`) "QueryOnly")
  (set `self.IsOn?` true)
  (goto _label :!via `PlayFromStart`))

(event `self.Trigger.OnComponentBeginOverlap`
  (params (OverlappedComponent :type "PrimitiveComponent Object Reference") (OtherActor :type "Actor Object Reference") (OtherComp :type "PrimitiveComponent Object Reference") (OtherBodyIndex :type Integer) (bFromSweep :type Boolean) (SweepResult :type "HitResult Structure (by ref)"))
  (cast `/Game/MyContent/Player/BP_PlayerBase` OtherActor)
  (`TimelineComponent.SetPlayRate` (`self.StandOn`) (`self.Stand Time`))
  (bind (_direction _alpha) (`Timeline|StandOn` :!via `PlayFromStart`)
    (:`Update`
      (`MaterialInstanceDynamic.SetScalarParameterValue` (`self.Material`) "Emissive" _alpha))
    (:`Finished`
      (`self.TurnOff`))))

(fn `UserConstructionScript`
  (bind _returnvalue (`PrimitiveComponent.CreateDynamicMaterialInstance` (`self.BaseFloor`) 0 "/Game/MyContent/GlobalMaterials/M_SuperGrid_SpecialPlatforms_Breaking.M_SuperGrid_SpecialPlatforms_Breaking" "None"))
  (set `self.Material` _returnvalue))