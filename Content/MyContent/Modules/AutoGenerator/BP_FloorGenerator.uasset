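; BP_FloorGenerator is a floor generator actor that adds one randomly typed floor piece on BeginPlay.
; GenerateFloors picks and prints a random floor type, then adds a child actor: static for Normal or Empty, dynamic for Breaking.
; The piece's Arrow world transform becomes the next SpawnTransform, allowing chaining, though it is applied as a relative transform and generation runs only once.
; Disconnected SpawnActor versions of the same logic remain unused.
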(event `self.ReceiveBeginPlay`
  (`self.GenerateFloors`))

(event `self.GenerateFloors`
  (bind (_spawn_transform_location _spawn_transform_rotation _spawn_transform_scale) (`KismetMathLibrary.BreakTransform` (`self.Spawn Transform`)))
  ;[0.2652 1 0.2584] Generator
  (bind _output_get (set `self.FloorType` (cast `/Game/MyContent/Modules/AutoGenerator/E_FloorType` (`KismetMathLibrary.Conv_IntToByte` (`KismetMathLibrary.RandomIntegerInRange` 0 2)))))
  ;;[1 0 0.04544] Debug
  (`KismetSystemLibrary.PrintString` (`KismetStringLibrary.Concat_StrStr` "Type: " (`|GetEnumeratorNameAsString` _output_get)) true true (struct :`R` 1.0 :`B` 0.045438 :`A` 1.0))
  (switch `/Game/MyContent/Modules/AutoGenerator/E_FloorType` _output_get
    (:`NewEnumerator0`
      (bind _returnvalue (`AddComponent|NODE_AddChildActorComponent-0` :`RelativeTransform` (`KismetMathLibrary.MakeTransform` _spawn_transform_location _spawn_transform_rotation _spawn_transform_scale) :!label _label))
      (`ChildActorComponent.SetChildActorClass` _returnvalue "/Game/MyContent/Modules/AutoGenerator/BP_BaseStaticFloor.BP_BaseStaticFloor_C")
      (bind _asbp_base_static_floor (cast `/Game/MyContent/Modules/AutoGenerator/BP_BaseStaticFloor` (`ChildActorComponent.ChildActor` _returnvalue)))
      (set `self.Spawn Transform` (`SceneComponent.K2_GetComponentToWorld` (`/Game/MyContent/Modules/AutoGenerator/BP_BaseStaticFloor.Arrow` _asbp_base_static_floor))))
    (:`NewEnumerator1`
      (goto _label))
    (:`NewEnumerator2`
      (bind _returnvalue_2 (`AddComponent|NODE_AddChildActorComponent-2` :`RelativeTransform` (`KismetMathLibrary.MakeTransform` _spawn_transform_location _spawn_transform_rotation _spawn_transform_scale)))
      (`ChildActorComponent.SetChildActorClass` _returnvalue_2 "/Game/MyContent/Modules/AutoGenerator/BP_BaseDynamicrFloor.BP_BaseDynamicrFloor_C")
      (bind _asbp_base_dynamicr_floor (cast `/Game/MyContent/Modules/AutoGenerator/BP_BaseDynamicrFloor` (`ChildActorComponent.ChildActor` _returnvalue_2)))
      (set `self.Spawn Transform` (`SceneComponent.K2_GetComponentToWorld` (`/Game/MyContent/Modules/AutoGenerator/BP_BaseDynamicrFloor.Arrow` _asbp_base_dynamicr_floor))))))

(fn `UserConstructionScript`)