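; BP_Walls_NoRoof_Black is a modular wall actor that, as its name suggests, has no roof and is sized in the editor through a size vector.
; The Construction Script scales both wall components in X and Z from that size, keeping Y thickness at 1.
; With Symmetry on, it offsets the Right component by the size to form the opposite side; otherwise it destroys the right wall.
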(fn `UserConstructionScript`
  (bind (_size_x _size_y) (`KismetMathLibrary.BreakVector` (`self.SIze`)))
  (bind (_returnvalue_x _returnvalue_y _returnvalue_z) (`KismetMathLibrary.BreakVector` (/ (`self.SIze`) 100.0)))
  (`|ExecutionSequence`
    (:`then_0`
      (`SceneComponent.SetRelativeScale3D` (`self.Wall_Left`) (`KismetMathLibrary.MakeVector` _returnvalue_x 1.0 _returnvalue_z))
      (`SceneComponent.SetRelativeScale3D` (`self.Wall_Right`) (`KismetMathLibrary.MakeVector` _returnvalue_x 1.0 _returnvalue_z)) ; Update walls scale
    )
    (:`then_2`
      (if (`self.Symmetry`)
        (`SceneComponent.K2_AddLocalOffset` (`self.Right`) (`KismetMathLibrary.MakeVector` (+ (* _size_x -1.0) 100.0) (* _size_y -1.0)) false false) ; Offset symmetric part
        (else
          (`ActorComponent.K2_DestroyComponent` (`self.Wall_Right`)))))))