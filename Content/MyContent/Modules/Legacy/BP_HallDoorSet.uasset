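; BP_HallDoorSet is a hall door that opens when a player enters its trigger box and closes when they leave, if movable.
; Box overlap events set the open state, call the open/close event and restart the opening clamp sound in both cases.
; A timeline, played forward or in reverse, drives the main door's relative Z position and plays the closing clamp sound when finished.
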(event `self.Box.OnComponentBeginOverlap`
  (params (OverlappedComponent :type "PrimitiveComponent Object Reference") (OtherActor :type "Actor Object Reference") (OtherComp :type "PrimitiveComponent Object Reference") (OtherBodyIndex :type Integer) (bFromSweep :type Boolean) (SweepResult :type "HitResult Structure (by ref)"))
  (bind _mechclampopen (`self.MechClampOpen`))
  (cast `/Game/MyContent/Player/BP_PlayerBase` OtherActor)
  (if (`self.IsMovable?`)
    (bind _output_get (set `self.IsOpen?` true))
    (`self.DoorOpen/Close` _output_get)
    (`AudioComponent.Stop` _mechclampopen :!label _label)
    (`AudioComponent.Play` _mechclampopen 0.0)))

(event `self.Box.OnComponentEndOverlap`
  (params (OverlappedComponent :type "PrimitiveComponent Object Reference") (OtherActor :type "Actor Object Reference") (OtherComp :type "PrimitiveComponent Object Reference") (OtherBodyIndex :type Integer))
  (cast `/Game/MyContent/Player/BP_PlayerBase` OtherActor)
  (if (`self.IsMovable?`)
    (bind _output_get (set `self.IsOpen?` false))
    (`self.DoorOpen/Close` _output_get)
    (goto _label)))

(event `DoorOpen/Close`
  (params (`Open?` :type Boolean))
  (bind _mechclampclose (`self.MechClampClose`))
  (bind _maindoor (`self.MainDoor`))
  (bind (_relativelocation_x _relativelocation_y) (`KismetMathLibrary.BreakVector` (`SceneComponent.RelativeLocation` _maindoor)))
  (if `Open?`
    (bind (_direction _locationz) (`Timeline|Timeline_0` :!via `PlayFromStart` :!label _label_2)
      (:`Update`
        (`SceneComponent.K2_SetRelativeLocation` _maindoor (`KismetMathLibrary.MakeVector` _relativelocation_x _relativelocation_y _locationz) false false))
      (:`Finished`
        (`AudioComponent.Stop` _mechclampclose)
        (`AudioComponent.Play` _mechclampclose 0.0)))
    (else
      (goto _label_2 :!via `ReverseFromEnd`))))

(fn `UserConstructionScript`)