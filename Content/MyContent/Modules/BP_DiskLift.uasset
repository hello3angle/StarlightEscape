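; BP_DiskLift is a lift module that moves its Parent component vertically in a repeating cycle from BeginPlay.
; Two chained timelines, LiftDown then LiftUp, set the relative Z to their curve value times EndPoint.Z, keeping X and Y.
; Lift calls itself when LiftUp finishes, checking IsMovable only at the start of each cycle.
; IsTimelineActive reports whether either timeline is playing.
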(event `self.ReceiveBeginPlay`
  (`self.Lift`))

(event `Lift`
  (bind _parent (`self.Parent`))
  (bind (_endpoint_x _endpoint_y _endpoint_z) (`KismetMathLibrary.BreakVector` (`self.EndPoint`)))
  (bind (_endpoint_x_2 _endpoint_y_2 _endpoint_z_2) (`KismetMathLibrary.BreakVector` (`self.EndPoint`)))
  (bind (_relativelocation_x _relativelocation_y) (`KismetMathLibrary.BreakVector` (`SceneComponent.RelativeLocation` _parent)))
  (if (`self.IsMovable?`)
    (bind (_direction _liftdownrate) (`Timeline|LiftDown` :!via `PlayFromStart`)
      (:`Update`
        (`SceneComponent.K2_SetRelativeLocation` _parent (`KismetMathLibrary.MakeVector` _relativelocation_x _relativelocation_y (* _liftdownrate _endpoint_z_2)) false false))
      (:`Finished`
        (bind (_direction_2 _liftuprate) (`Timeline|LiftUp` :!via `PlayFromStart`)
          (:`Update`
            (`SceneComponent.K2_SetRelativeLocation` _parent (`KismetMathLibrary.MakeVector` _relativelocation_x _relativelocation_y (* _liftuprate _endpoint_z)) false false))
          (:`Finished`
            (`self.Lift`)))))))

(fn `IsTimelineActive?`
  (returns (`IsTimelineActive?` :type Boolean))
  (return (or (`ActorComponent.IsActive` (`self.LiftDown`)) (`ActorComponent.IsActive` (`self.LiftUp`)))))

(fn `UserConstructionScript`)