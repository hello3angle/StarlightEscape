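; Moving platform that shuttles between its origin and the Platform component's relative location, starting on BeginPlay when Enabled.
; A timeline lerps PlatformTransform's relative location, with play rate set to 1 / MoveSpeed, so larger values move slower.
; A FlipFlop on timeline completion alternates forward and reverse playback, pausing for DelayTime before each trip.
; Reveal and Hide events toggle MovingPlatform's visibility and collision (query-only or none).
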(event `self.ReceiveBeginPlay`
  ;[1 1 1] Begin Play
  (`parent.ReceiveBeginPlay`)
  (if (`self.Enabled`)
    (`self.MovePlatform`)))

(event `PlayForward`
  ;[1 1 1] Move Platform Back and Forth
  (`KismetSystemLibrary.Delay` (`self.DelayTime`))
  (bind (_direction _alpha) (`Timeline|MovePlatform_TL` :!label _label)
    (:`Update`
      (`SceneComponent.K2_SetRelativeLocation` (`self.PlatformTransform`) (`KismetMathLibrary.VLerp` (0.0 0.0 0.0) (`SceneComponent.RelativeLocation` (`self.Platform`)) _alpha) false false))
    (:`Finished`
      (`/Engine/EditorBlueprintResources/StandardMacros.FlipFlop`
        (:`A`
          (`self.PlayReverse`))
        (:`B`
          (`self.PlayForward`))))))

(event `PlayReverse`
  ;[1 1 1] Move Platform Back and Forth
  (`KismetSystemLibrary.Delay` (`self.DelayTime`))
  (goto _label :!via `Reverse`))

(event `MovePlatform`
  ;[1 1 1] Begin Moving the Platform
  (`TimelineComponent.SetPlayRate` (`self.MovePlatform_TL`) (/ 1.0 (`self.MoveSpeed`)))
  (`self.PlayForward`))

(event `/Game/MyContent/Platforms/BI_Platforms.RevealPlatform`
  (bind _movingplatform (`self.MovingPlatform`))
  (`SceneComponent.SetVisibility` _movingplatform true true)
  (`PrimitiveComponent.SetCollisionEnabled` _movingplatform "QueryOnly"))

(event `/Game/MyContent/Platforms/BI_Platforms.HidePlatform`
  (bind _movingplatform (`self.MovingPlatform`))
  (`SceneComponent.SetVisibility` _movingplatform false true)
  (`PrimitiveComponent.SetCollisionEnabled` _movingplatform "NoCollision"))

(fn `UserConstructionScript`
  (`parent.UserConstructionScript`))