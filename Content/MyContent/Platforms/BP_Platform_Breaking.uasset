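; Breaking platform that gives way shortly after being stepped on, then respawns.
; Trigger overlap plays a once-per-cycle sound with random pitch and starts a StandTime-scaled timeline that brightens the material's emissive.
; When it finishes, collision turns off and a shared hide/respawn timeline reverses to drive the appearance parameter.
; After RespawnTime, TurnOn restores collision, glow and sound gate; the IsOn check stops the forward playback from retriggering respawn.
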(event `self.Trigger.OnComponentBeginOverlap`
  (params (OverlappedComponent :type "PrimitiveComponent Object Reference") (OtherActor :type "Actor Object Reference") (OtherComp :type "PrimitiveComponent Object Reference") (OtherBodyIndex :type Integer) (bFromSweep :type Boolean) (SweepResult :type "HitResult Structure (by ref)"))
  (`|ExecutionSequence`
    (:`then_0`
      (`TimelineComponent.SetPlayRate` (`self.StandOn`) (/ 1.0 (`self.StandTime`)))
      (bind (_direction _alpha) (`Timeline|StandOn` :!via `PlayFromStart`)
        (:`Update`
          (`MaterialInstanceDynamic.SetScalarParameterValue` (`self.Material`) "Emissive" _alpha))
        (:`Finished`
          (`self.TurnOff`))))
    (:`then_1`
      (`/Engine/EditorBlueprintResources/StandardMacros.DoOnce` false :!label _label
        (:`Completed`
          (`GameplayStatics.PlaySoundAtLocation` "/Game/MyContent/Audio/AC_StepOnBreaking.AC_StepOnBreaking" (`self.K2_GetActorLocation`) (struct) 1.0 (`KismetMathLibrary.RandomFloatInRange` 0.8 1.15) 0.0 null null null null))))))

(event `ResetSound`
  (goto _label :!via `Reset`))

(event `TurnOff`
  ;[1 1 1] Turn Platform on /off
  (`PrimitiveComponent.SetCollisionEnabled` (`self.Trigger`) "NoCollision")
  (`PrimitiveComponent.SetCollisionEnabled` (`self.Platform`) "NoCollision")
  (set `self.IsOn?` false)
  (bind (_direction _alpha) (`Timeline|HideandRespawnTL` :!via `ReverseFromEnd` :!label _label_2)
    (:`Update`
      (`MaterialInstanceDynamic.SetScalarParameterValue` (`self.Material`) "Appearence" _alpha))
    (:`Finished`
      (`KismetSystemLibrary.Delay` (`self.RespawnTime`))
      (if (not (`self.IsOn?`))
        (`self.TurnOn`)))))

(event `TurnOn`
  ;[1 1 1] Turn Platform on /off
  (`self.ResetSound`)
  (`MaterialInstanceDynamic.SetScalarParameterValue` (`self.Material`) "Emissive" 0.0)
  (`PrimitiveComponent.SetCollisionEnabled` (`self.Platform`) "QueryAndPhysics")
  (`PrimitiveComponent.SetCollisionEnabled` (`self.Trigger`) "QueryOnly")
  (set `self.IsOn?` true)
  (goto _label_2 :!via `PlayFromStart`))

(fn `UserConstructionScript`
  (`parent.UserConstructionScript`))