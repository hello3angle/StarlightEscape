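; BP_Platform is a resizable platform actor that can be revealed and hidden at runtime.
; RevealPlatform shows it with query-only collision and plays a timeline driving the "Appearence" material parameter, while HidePlatform instantly hides it, disables collision and resets that parameter.
; The construction script scales the mesh from Size divided by 100 and creates a dynamic material whose X/Y pattern parameters follow Size.
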(event `/Game/MyContent/Platforms/BI_Platforms.RevealPlatform`
  (`SceneComponent.SetVisibility` (`self.Platform`) true true)
  (`PrimitiveComponent.SetCollisionEnabled` (`self.Platform`) "QueryOnly")
  (bind (_direction _alpha) (`Timeline|Appear_TL` :!via `PlayFromStart`)
    (:`Update`
      (`MeshComponent.SetScalarParameterValueOnMaterials` (`self.Platform`) "Appearence" _alpha))))

(event `/Game/MyContent/Platforms/BI_Platforms.HidePlatform`
  (`SceneComponent.SetVisibility` (`self.Platform`) false true)
  (`PrimitiveComponent.SetCollisionEnabled` (`self.Platform`) "NoCollision")
  (`MeshComponent.SetScalarParameterValueOnMaterials` (`self.Platform`) "Appearence" 0.0))

(fn `GetNormalSize`
  (returns (NormalizedSize :type "Vector Structure"))
  (bind (_returnvalue_x _returnvalue_y _returnvalue_z) (`KismetMathLibrary.BreakVector` (/ (`self.Size`) 100.0)))
  (return (`KismetMathLibrary.MakeVector` _returnvalue_x _returnvalue_y _returnvalue_z)))

(fn `UserConstructionScript`
  (bind (_size_x _size_y) (`KismetMathLibrary.BreakVector` (`self.Size`)))
  (`SceneComponent.SetRelativeScale3D` (`self.Platform`) (`self.GetNormalSize`))
  (bind _returnvalue (`PrimitiveComponent.CreateDynamicMaterialInstance` (`self.Platform`) 0 (`PrimitiveComponent.GetMaterial` (`self.Platform`) 0) "None"))
  (bind _output_get (set `self.Material` _returnvalue))
  (`MaterialInstanceDynamic.SetScalarParameterValue` _output_get "PatternX" (/ _size_x 2.0))
  (`MaterialInstanceDynamic.SetScalarParameterValue` (`self.Material`) "PatternY" (/ _size_y 2.0)))