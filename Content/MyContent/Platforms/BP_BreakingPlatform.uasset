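; BP_BreakingPlatform is a platform that disappears shortly after something overlaps its trigger, then respawns.
; An overlap on Trigger waits StandTime, then HideAndRespawn disables collision on both components and hides the platform mesh.
; After RespawnTime it restores physics collision on Platform, query-only collision on Trigger, and visibility.
; The overlap has no filter on which actor starts it.
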(event `self.Trigger.OnComponentBeginOverlap`
  (params (OverlappedComponent :type "PrimitiveComponent Object Reference") (OtherActor :type "Actor Object Reference") (OtherComp :type "PrimitiveComponent Object Reference") (OtherBodyIndex :type Integer) (bFromSweep :type Boolean) (SweepResult :type "HitResult Structure (by ref)"))
  (`KismetSystemLibrary.Delay` (`self.StandTime`))
  (`self.HideAndRespawn`))

(event `HideAndRespawn`
  (`PrimitiveComponent.SetCollisionEnabled` (`self.Trigger`) "NoCollision")
  (`PrimitiveComponent.SetCollisionEnabled` (`self.Platform`) "NoCollision")
  (`SceneComponent.SetVisibility` (`self.Platform`) false true)
  (`KismetSystemLibrary.Delay` (`self.RespawnTime`))
  (`PrimitiveComponent.SetCollisionEnabled` (`self.Platform`) "QueryAndPhysics")
  (`PrimitiveComponent.SetCollisionEnabled` (`self.Trigger`) "QueryOnly")
  (`SceneComponent.SetVisibility` (`self.Platform`) true true))

(fn `UserConstructionScript`)