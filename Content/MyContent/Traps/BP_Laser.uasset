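; BP_Laser is a laser trap that sends death and kill-player messages to any actor overlapping its box trigger.
; The construction script sets the Niagara beam end at MaxRange along the actor's forward vector.
; On BeginPlay, a single visibility trace along the cylinder's negative up axis moves the beam end to any hit.
; The box is resized and offset to span the hit distance, or MaxRange when nothing is hit.
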(event `self.ReceiveBeginPlay`
  (`self.SetBeamEnd`))

(event `self.Box.OnComponentBeginOverlap`
  (params (OverlappedComponent :type "PrimitiveComponent Object Reference") (OtherActor :type "Actor Object Reference") (OtherComp :type "PrimitiveComponent Object Reference") (OtherBodyIndex :type Integer) (bFromSweep :type Boolean) (SweepResult :type "HitResult Structure (by ref)"))
  ;[1 1 1] Kill player if they overlap it
  (message `/Game/MyContent/Player/Settings/BI_PlayerInteractions.LaserDeath` OtherActor)
  (message `/Game/MyContent/Player/Settings/BI_PlayerInteractions.KillPlayer` OtherActor))

(fn `SetBeamEnd`
  (bind _cylinder (`self.Cylinder`))
  (bind _returnvalue (`SceneComponent.K2_GetComponentLocation` _cylinder))
  (bind (_returnvalue_x _returnvalue_y _returnvalue_z) (`KismetMathLibrary.BreakVector` (`BoxComponent.GetScaledBoxExtent` (`self.Box`))))
  (bind (_returnvalue_x_2 _returnvalue_y_2 _returnvalue_z_2) (`KismetMathLibrary.BreakVector` (`BoxComponent.GetScaledBoxExtent` (`self.Box`))))
  (bind (_outhit _returnvalue_2) (`KismetSystemLibrary.LineTraceSingle` :`Start` _returnvalue :`End` (+ _returnvalue (* (`KismetMathLibrary.NegateVector` (`SceneComponent.GetUpVector` _cylinder)) (`self.MaxRange`))) :`TraceChannel` "TraceTypeQuery1" :`TraceColor` (struct :`G` 0.239506 :`B` 1.0 :`A` 1.0)))
  (if _returnvalue_2
    (`|ExecutionSequence`
      (:`then_0`
        (bind (_bblockinghit _binitialoverlap _time _distance _location) (`GameplayStatics.BreakHitResult` _outhit))
        (`FXSystemComponent.SetVectorParameter` (`self.Niagara`) "User.Beam End" _location))
      (:`then_1`
        (bind _returnvalue_3 (/ _distance 2.0))
        (`BoxComponent.SetBoxExtent` (`self.Box`) (`KismetMathLibrary.MakeVector` _returnvalue_3 _returnvalue_y_2 _returnvalue_z_2) true)
        (bind _result (`/Engine/EditorBlueprintResources/StandardMacros.NegateFloat` _returnvalue_3)
          (:`  `
            (`SceneComponent.K2_SetRelativeLocation` (`self.Box`) (`KismetMathLibrary.MakeVector` 0.0 0.0 _result) false false)))))
    (else
      (`BoxComponent.SetBoxExtent` (`self.Box`) (`KismetMathLibrary.MakeVector` (/ (`self.MaxRange`) 2.0) _returnvalue_y _returnvalue_z) true)
      (bind _result_2 (`/Engine/EditorBlueprintResources/StandardMacros.NegateFloat` (/ (`self.MaxRange`) 2.0))
        (:`  `
          (`SceneComponent.K2_SetRelativeLocation` (`self.Box`) (`KismetMathLibrary.MakeVector` 0.0 0.0 _result_2) false false))))))

(fn `UserConstructionScript`
  (`FXSystemComponent.SetVectorParameter` (`self.Niagara`) "User.Beam End" (+ (`SceneComponent.K2_GetComponentLocation` (`self.Cylinder`)) (* (`self.GetActorForwardVector`) (`self.MaxRange`)))))