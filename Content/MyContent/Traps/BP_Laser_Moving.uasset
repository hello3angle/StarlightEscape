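; Moving laser trap that slides its Cylinder back and forth between its local origin and an EndPoint component.
; On BeginPlay it runs the parent logic, sets the timeline play rate from MoveSpeed and starts moving.
; The timeline lerps the relative location, and a FlipFlop on finish alternates forward and reverse runs, each preceded by DelayTime.
; Tick calls SetBeamEnd every frame to update the beam.
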(event `self.ReceiveBeginPlay`
  ;[1 1 1] Begin Play
  (`parent.ReceiveBeginPlay`)
  (`self.MoveLaser`))

(event `PlayForward`
  ;[1 1 1] Move Platform Back and Forth
  (`KismetSystemLibrary.Delay` (`self.DelayTime`))
  (bind (_direction _alpha) (`Timeline|MoveLaser_TL` :!label _label)
    (:`Update`
      (`SceneComponent.K2_SetRelativeLocation` (`self.Cylinder`) (`KismetMathLibrary.VLerp` (0.0 0.0 0.0) (`SceneComponent.RelativeLocation` (`self.EndPoint`)) _alpha) false false))
    (:`Finished`
      (`/Engine/EditorBlueprintResources/StandardMacros.FlipFlop`
        (:`A`
          (`self.PlayReverse`))
        (:`B`
          (`self.PlayForward`))))))

(event `PlayReverse`
  ;[1 1 1] Move Platform Back and Forth
  (`KismetSystemLibrary.Delay` (`self.DelayTime`))
  (goto _label :!via `ReverseFromEnd`))

(event `MoveLaser`
  ;[1 1 1] Begin Moving the Platform
  (`TimelineComponent.SetPlayRate` (`self.MoveLaser_TL`) (/ 1.0 (`self.MoveSpeed`)))
  (`self.PlayForward`))

(event `self.ReceiveTick`
  (params (DeltaSeconds :type "Float (single-precision)"))
  (`self.SetBeamEnd`))

(fn `UserConstructionScript`
  (`parent.UserConstructionScript`))