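; BP_PushTrap is a trap that periodically switches on and off and launches Characters that touch it while it is active.
; From BeginPlay, ActivateTrap and DeactivateTrap call each other after an OnOffTime delay, swapping the TrapMesh material and toggling PushCollision between query-only and no collision.
; Overlapping PushCollision launches the Character along that component's forward vector, scaled by LaunchPower and added to its current velocity.
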(event `self.ReceiveBeginPlay`
  ;[1 1 1] begin play
  (`self.ActivateTrap`))

(event `ActivateTrap`
  ;[1 1 1] Activate / Deactivate Trap
  (`PrimitiveComponent.SetMaterial` (`self.TrapMesh`) 0 "/Engine/MapTemplates/Materials/BasicAsset01.BasicAsset01")
  (`PrimitiveComponent.SetCollisionEnabled` (`self.PushCollision`) "QueryOnly")
  (`KismetSystemLibrary.Delay` (`self.On/OffTime`))
  (`self.DeactivateTrap`))

(event `DeactivateTrap`
  ;[1 1 1] Activate / Deactivate Trap
  (`PrimitiveComponent.SetMaterial` (`self.TrapMesh`) 0 "/Engine/MapTemplates/Materials/BasicAsset03.BasicAsset03")
  (`PrimitiveComponent.SetCollisionEnabled` (`self.PushCollision`) "NoCollision")
  (`KismetSystemLibrary.Delay` (`self.On/OffTime`))
  (`self.ActivateTrap`))

(event `self.PushCollision.OnComponentBeginOverlap`
  (params (OverlappedComponent :type "PrimitiveComponent Object Reference") (OtherActor :type "Actor Object Reference") (OtherComp :type "PrimitiveComponent Object Reference") (OtherBodyIndex :type Integer) (bFromSweep :type Boolean) (SweepResult :type "HitResult Structure (by ref)"))
  ;[1 1 1] lauch Character away from trap
  (bind _ascharacter (cast `Character` OtherActor))
  (`Character.LaunchCharacter` _ascharacter (* (`SceneComponent.GetForwardVector` (`self.PushCollision`)) (`self.LaunchPower`)) false false))

(fn `UserConstructionScript`)