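; BP_LaserGate is a trap with top and bottom laser child actors, each of which can be disabled.
; On BeginPlay it destroys the disabled laser components and passes LaserLength as max range to child actors via SetMaxRangeMessage.
; When only the top laser is disabled, that call targets the destroyed TopLaser, so BottomLaser never receives the length.
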(event `self.ReceiveBeginPlay`
  (bind _laserlength (`self.LaserLength`))
  (if (`self.DisableTopLaser?`)
    (`ActorComponent.K2_DestroyComponent` (`self.TopLaser`))
    (if (`self.DisableBottomLaser?`)
      (`ActorComponent.K2_DestroyComponent` (`self.BottomLaser`))
      (else
        (message `/Game/MyContent/Traps/BI_Laser.SetMaxRange` (`ChildActorComponent.ChildActor` (`self.TopLaser`)) (`self.LaserLength`))))
    (elif (`self.DisableBottomLaser?`)
      (`ActorComponent.K2_DestroyComponent` (`self.BottomLaser`))
      (message `/Game/MyContent/Traps/BI_Laser.SetMaxRange` (`ChildActorComponent.ChildActor` (`self.TopLaser`)) (`self.LaserLength`))
      (else
        (message `/Game/MyContent/Traps/BI_Laser.SetMaxRange` (`ChildActorComponent.ChildActor` (`self.BottomLaser`)) _laserlength)
        (message `/Game/MyContent/Traps/BI_Laser.SetMaxRange` (`ChildActorComponent.ChildActor` (`self.TopLaser`)) _laserlength)))))

(fn `UserConstructionScript`)