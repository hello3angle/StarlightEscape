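; BP_FallingAsteroid is a trap: a randomly scaled asteroid moved by a projectile movement component that kills the player on contact.
; Each tick, a downward line trace from the mesh places a decal just above the surface below, marking the spot beneath it.
; A mesh hit sends KillPlayerMessage to the struck actor and enables the Sphere's collision, whose overlaps send the same message.
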(event `self.ReceiveTick`
  (params (DeltaSeconds :type "Float (single-precision)"))
  (bind _returnvalue (`SceneComponent.K2_GetComponentLocation` (`self.SM_Asteroid_01`)))
  (bind (_outhit _returnvalue_2) (`KismetSystemLibrary.LineTraceSingle` _returnvalue (+ _returnvalue (* (`KismetMathLibrary.Vector_Down`) (`self.LineTraceLength`))) "TraceTypeQuery1"))
  (if _returnvalue_2
    (`SceneComponent.K2_SetWorldLocation` (`self.Decal`) (+ (`.ImpactPoint` (`GameplayStatics.BreakHitResult` _outhit)) (0.0 0.0 5.0)) false false)
    (`SceneComponent.K2_SetWorldRotation` (`self.Decal`) (struct :`Pitch` 90.0) false false)))

(event `self.SM_Asteroid_01.OnComponentHit`
  (params (HitComponent :type "PrimitiveComponent Object Reference") (OtherActor :type "Actor Object Reference") (OtherComp :type "PrimitiveComponent Object Reference") (NormalImpulse :type "Vector Structure") (Hit :type "HitResult Structure (by ref)"))
  (message `/Game/MyContent/Player/Settings/BI_PlayerInteractions.KillPlayer` OtherActor)
  (`PrimitiveComponent.SetCollisionEnabled` (`self.Sphere`) "QueryAndPhysics"))

(event `self.Sphere.OnComponentBeginOverlap`
  (params (OverlappedComponent :type "PrimitiveComponent Object Reference") (OtherActor :type "Actor Object Reference") (OtherComp :type "PrimitiveComponent Object Reference") (OtherBodyIndex :type Integer) (bFromSweep :type Boolean) (SweepResult :type "HitResult Structure (by ref)"))
  (message `/Game/MyContent/Player/Settings/BI_PlayerInteractions.KillPlayer` OtherActor))

(fn `UserConstructionScript`
  (bind _returnvalue (`KismetMathLibrary.RandomFloatInRange` 0.5 1.0))
  (`SceneComponent.SetWorldScale3D` (`self.SM_Asteroid_01`) (`KismetMathLibrary.MakeVector` _returnvalue _returnvalue _returnvalue))
  (set `MovementComponent.Velocity` (0.0 0.0 10.0) (`self.ProjectileMovement`)))