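; BP_AsteroidSpawner is a trap actor that repeatedly spawns BP_FallingAsteroid high above its own location, passing along minimum and maximum size.
; While SpawnAsteroids is true, BeginPlay starts the cycle after a random delay, and SpawnAsteroid calls itself again after a longer random delay.
; ToggleAsteroidSpawn sets the flag and starts a new delayed spawn when turned on; turning it off does not cancel a pending spawn.
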(event `self.ReceiveBeginPlay`
  (if (`self.SpawnAsteroids?`)
    (`KismetSystemLibrary.Delay` (`KismetMathLibrary.RandomFloatInRange` 2.0 8.0))
    (`self.Spawn Asteroid`)))

(event `Spawn Asteroid`
  (bind (_returnvalue_location _returnvalue_rotation _returnvalue_scale) (`KismetMathLibrary.BreakTransform` (`self.GetTransform`)))
  (`|SpawnActorFromClass` "/Game/MyContent/Traps/FallingAsteroid/BP_FallingAsteroid.BP_FallingAsteroid_C" (`KismetMathLibrary.MakeTransform` (+ _returnvalue_location (0.0 0.0 5000.0)) _returnvalue_rotation _returnvalue_scale) "Undefined" "OverrideRootScale" null (`self.Min Size`) (`self.Max Size`) null)
  (if (`self.SpawnAsteroids?`)
    (`KismetSystemLibrary.Delay` (`KismetMathLibrary.RandomFloatInRange` 5.0 15.0))
    (`self.Spawn Asteroid`)))

(event `/Game/MyContent/Traps/FallingAsteroid/BI_AsteroidTrap.ToggleAsteroidSpawn`
  (params (`TurnOn/Off` :type Boolean))
  (bind _output_get (set `self.SpawnAsteroids?` `TurnOn/Off`))
  (if _output_get
    (`KismetSystemLibrary.Delay` (`KismetMathLibrary.RandomFloatInRange` 2.0 8.0))
    (`self.Spawn Asteroid`)))

(fn `UserConstructionScript`)