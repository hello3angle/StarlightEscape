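; BP_FallingAsteroid is a falling asteroid trap that marks its impact area with a warning decal found by a downward line trace.
; Construction randomizes collision sphere scale, blast radius, decal size and fall speed, each rolled separately.
; On hit it plays explosion effects, sends a kill message to a Pawn found by a sphere trace, then destroys itself and the decal.
; A Reset event holds delayed respawn logic, but the hit path never calls it.
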(event `self.ReceiveBeginPlay`
  ;[1 1 1] begin play
  (`self.PlaceDecal`))

(event `PlaceDecal`
  (bind _returnvalue (`SceneComponent.K2_GetComponentLocation` (`self.Sphere`)))
  ;[1 1 1] Place a warning decal onto floor of impact area
  (bind (_outhit _returnvalue_2) (`KismetSystemLibrary.LineTraceSingle` _returnvalue (+ _returnvalue (* (`KismetMathLibrary.Vector_Down`) (`self.LineTraceLength`))) "TraceTypeQuery1"))
  (if _returnvalue_2
    (bind _returnvalue_3 (`GameplayStatics.SpawnDecalAtLocation` "/Game/MyContent/Traps/M_FallArea.M_FallArea" (`self.DecalSize`) (+ (`.ImpactPoint` (`GameplayStatics.BreakHitResult` _outhit)) (0.0 0.0 5.0)) (struct :`Pitch` 90.0)))
    (set `self.DecalPlaced` _returnvalue_3)))

(event `self.Sphere.OnComponentHit`
  (params (HitComponent :type "PrimitiveComponent Object Reference") (OtherActor :type "Actor Object Reference") (OtherComp :type "PrimitiveComponent Object Reference") (NormalImpulse :type "Vector Structure") (Hit :type "HitResult Structure (by ref)"))
  (bind _returnvalue (`self.K2_GetActorLocation`))
  (bind _returnvalue_2 (`self.K2_GetActorLocation`))
  (`|ExecutionSequence`
    (:`then_0`
      ;[1 1 1] Spawn Sound
      (`GameplayStatics.SpawnSoundAtLocation` "/Game/MyContent/Audio/AC_FireExplode.AC_FireExplode" _returnvalue (struct) 0.8 1.0 0.0 "/Game/MyContent/Audio/AT_FireExplode.AT_FireExplode" null)
      ;[1 1 1] Explosion
      (`GameplayStatics.SpawnEmitterAtLocation` "/Game/Luos8Elements/Particles/Fire/Par_LMagic_Fire_Explosion_Xdir.Par_LMagic_Fire_Explosion_Xdir" (+ _returnvalue (0.0 0.0 20.0)) (`self.K2_GetActorRotation`) (2.0 2.0 2.0))
      ;[1 1 1] Deactivate flying particle.
      (`ActorComponent.Deactivate` (`self.MovingParticle`))
      ;[1 1 1] Check if player Was in Area if so Kill them
      (bind (_outhit _returnvalue_3) (`KismetSystemLibrary.SphereTraceSingleForObjects` _returnvalue_2 _returnvalue_2 (`self.BlastRadius`) (`|MakeArray` "ObjectTypeQuery3" :!type "EObjectTypeQuery Enum")))
      (if _returnvalue_3
        (message `/Game/MyContent/Player/Settings/BI_PlayerInteractions.KillPlayer` (`.HitActor` (`GameplayStatics.BreakHitResult` _outhit)))))
    (:`then_1`
      (bind _decalplaced (`self.DecalPlaced`)
        (:`then`
          (`ActorComponent.K2_DestroyComponent` _decalplaced))
        (:`else`
          _))
      (`self.K2_DestroyActor`))))

(event `Reset`
  (bind _sm_asteroid_01 (`self.SM_Asteroid_01`))
  (bind _sm_asteroid_01_2 (`self.SM_Asteroid_01`))
  (bind _sm_asteroid_01_3 (`self.SM_Asteroid_01`))
  (`/Engine/EditorBlueprintResources/StandardMacros.DoOnce` false :!via `Reset`
    (:`Completed`
      (`AudioComponent.Stop` (`self.Audio`))
      ;[1 1 1] Turn Asteroid Off, Delay Then Restart
      (`SceneComponent.SetVisibility` (`self.SM_Asteroid_01`) false false)
      (`PrimitiveComponent.SetSimulatePhysics` (`self.SM_Asteroid_01`) false)
      (`PrimitiveComponent.SetEnableGravity` _sm_asteroid_01_2 false)
      (`PrimitiveComponent.SetCollisionEnabled` _sm_asteroid_01_2 "NoCollision")
      (`KismetSystemLibrary.Delay` (`KismetMathLibrary.RandomFloatInRange` 8.0 20.0))
      (`self.K2_SetActorLocation` (`self.StartLoc`))
      (`self.RandomSizeAsteroid`)
      (`SceneComponent.SetVisibility` _sm_asteroid_01 true false)
      (`PrimitiveComponent.SetCollisionEnabled` _sm_asteroid_01 "QueryAndPhysics")
      (`PrimitiveComponent.SetSimulatePhysics` _sm_asteroid_01_3 true)
      (`PrimitiveComponent.SetEnableGravity` _sm_asteroid_01_3 true)
      (`ActorComponent.Activate` (`self.MovingParticle`) true)
      (`self.PlaceDecal`)
      (`self.Reset`)
      (`AudioComponent.Play` (`self.Audio`) 0.0))))

(fn `RandomSizeAsteroid`
  (bind _returnvalue (`KismetMathLibrary.RandomFloatInRange` (`self.MinSize`) (`self.MaxSize`)))
  (bind (_returnvalue_x _returnvalue_y _returnvalue_z) (`KismetMathLibrary.BreakVector` (* _returnvalue (`self.BaseDecalSize`))))
  (set `self.BlastRadius` (* (`self.BaseBlastRadius`) _returnvalue))
  (`SceneComponent.SetWorldScale3D` (`self.Sphere`) (`KismetMathLibrary.MakeVector` _returnvalue _returnvalue _returnvalue))
  (set `self.DecalSize` (`KismetMathLibrary.MakeVector` 50.0 _returnvalue_y _returnvalue_z))
  (set `MovementComponent.Velocity` (`KismetMathLibrary.MakeVector` 0.0 0.0 (`KismetMathLibrary.RandomFloatInRange` -1000.0 -1500.0)) (`self.ProjectileMovement`)))

(fn `UserConstructionScript`
  (`self.RandomSizeAsteroid`)
  (set `self.StartLoc` (`self.K2_GetActorLocation`)))