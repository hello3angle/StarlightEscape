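; BP_GameModeBase is a game mode Blueprint that keeps a running player time as a Timespan.
; StartTimer sets a looping one-second timer that calls the Time function to add a second to PlayersTime, and stores its handle in PlayerTimer.
; PauseTimer and ResumeTimer act on that handle, while AddTime and SubtractTime adjust the total by a given number of seconds.
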(event `self.ReceiveTick`
  (params (DeltaSeconds :type "Float (single-precision)")))

(event `StartTimer`
  (bind _returnvalue (`KismetSystemLibrary.K2_SetTimer` null "Time" 1.0 true))
  (set `self.PlayerTimer` _returnvalue))

(event `PauseTimer`
  (`KismetSystemLibrary.K2_PauseTimerHandle` (`self.PlayerTimer`)))

(event `ResumeTimer`
  (`KismetSystemLibrary.K2_UnPauseTimerHandle` (`self.PlayerTimer`)))

(event `AddTime`
  (params (Seconds :type Integer))
  (set `self.PlayersTime` (+ (`self.PlayersTime`) (`KismetMathLibrary.MakeTimespan` 0 0 0 Seconds))))

(event `SubtractTime`
  (params (Seconds :type Integer))
  (set `self.PlayersTime` (- (`self.PlayersTime`) (`KismetMathLibrary.MakeTimespan` 0 0 0 Seconds))))

(fn `Time`
  (set `self.PlayersTime` (+ (`self.PlayersTime`) (`KismetMathLibrary.MakeTimespan` 0 0 0 1)))
  (return))

(fn `UserConstructionScript`)