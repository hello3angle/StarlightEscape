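; Base player character Blueprint handling movement, camera input, death and checkpoint respawn, HUD and pause menu.
; Movement adds a stamina-gated double jump fed by timer regeneration, a montage-driven slide, and a cooldown launch dash with dynamic-material effect.
; Death and reset share a path that fades appearance through mesh parameters and a parameter collection, then teleports to the stored spawn point.
; Number keys provide debug teleports and pause.
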(event `self.ReceiveBeginPlay`
  (bind _charactermovement (`self.CharacterMovement`))
  (bind _returnvalue (`SceneComponent.K2_GetComponentLocation` (`self.CapsuleComponent`)))
  ;[0.2652 1 0.2584] Set Movement DefaultValues
  (set `CharacterMovementComponent.MaxWalkSpeed` (`self.RunSpeed`) _charactermovement)
  (set `CharacterMovementComponent.MaxWalkSpeedCrouched` (`self.CrouchSpeed`) _charactermovement)
  (set `CharacterMovementComponent.JumpZVelocity` (`self.JumpZVelocity`) _charactermovement)
  (set `CharacterMovementComponent.MaxAcceleration` (`self.Acceleration`) _charactermovement)
  ;[0.175 0.2754 1] Set Capsule Height
  (set `CharacterMovementComponent.CrouchedHalfHeight` (`self.CrouchedHeight`) _charactermovement)
  (`CapsuleComponent.SetCapsuleHalfHeight` (`self.CapsuleComponent`) (`self.CapsuleHeight`) true)
  ;[0.175 0.2754 1] Dash VFX Material
  (bind _returnvalue_2 (`PrimitiveComponent.CreateDynamicMaterialInstance` (`self.Mesh`) 0 null "None"))
  (set `self.DashMat Ref` _returnvalue_2)
  ;[0.175 0.2754 1] Set StaminaRegen
  (`KismetSystemLibrary.K2_SetTimer` null "RegenStamina" (`self.StaminaRegenInterval`) true)
  (`self.SetUI`)
  ;[0.175 0.2754 1] Widget - FadeScreen
  (`|ExecutionSequence`
    (:`then_0`
      (bind _returnvalue_3 (`|CreateWidget` "/Game/MyContent/Widgets/WS_FadeScreen.WS_FadeScreen_C"))
      (bind _output_get (set `self.FadeWidget Ref` _returnvalue_3))
      (`UserWidget.AddToViewport` _output_get 0))
    (:`then_1`
      ;[1 0.1562 0.1562] Tutorial Cinematic Screen
      (if (`self.IsTutorial?`)
        (bind _outhit (`KismetSystemLibrary.LineTraceSingleForObjects` _returnvalue (+ _returnvalue (1.0 0.0 0.0)) (`self.InitialTraceObjects`)))
        (bind _asbp_dialogue_actor (cast `/Game/MyContent/Dialogues/BP_DialogueActor` (`.HitActor` (`GameplayStatics.BreakHitResult` _outhit))))
        (message `/Game/MyContent/Dialogues/BI_DialogueInteractions.ShowDialogue` _asbp_dialogue_actor)))
    (:`then_2`
      (`/Game/MyContent/Widgets/WS_FadeScreen.FadeIn` (`self.FadeWidget Ref`)))))

(event `/Game/MyContent/Player/Settings/BI_PlayerInteractions.SetPlayerRespawnPoint`
  (params (Respawn :type "Transform Structure"))
  ;[1 1 1] Set Respawn Point
  (set `self.SpawnPoint` Respawn))

(event `/Game/MyContent/Player/Settings/BI_PlayerControls.MoveForward/Backward`
  (params (Axis :type "Float (double-precision)"))
  (bind (_returnvalue_roll _returnvalue_pitch _returnvalue_yaw) (`KismetMathLibrary.BreakRotator` (`self.GetControlRotation`)))
  ;[0.2652 1 0.2584] Movement
  (`self.AddMovementInput` (`KismetMathLibrary.GetForwardVector` (`KismetMathLibrary.MakeRotator` 0.0 0.0 _returnvalue_yaw)) Axis))

(event `EnableInputKeys`
  ;[1 0.1562 0.1562] Show Intro Scene
  (`self.EnableInput` (`GameplayStatics.GetPlayerController` 0) null))

(event `Respawn`
  (bind (_spawnpoint_location _spawnpoint_rotation) (`KismetMathLibrary.BreakTransform` (`self.SpawnPoint`)))
  ;[1 1 1] Respawn
  ;;[1 1 1] Move player to spawn point
  (`self.K2_SetActorTransform` (`KismetMathLibrary.MakeTransform` _spawnpoint_location _spawnpoint_rotation) false true)
  (bind (_direction _alpha) (`Timeline|Timeline_1` :!via `PlayFromStart`)
    (:`Update`
      (`MeshComponent.SetScalarParameterValueOnMaterials` (`self.Mesh`) "Appearence" _alpha)
      (`KismetMaterialLibrary.SetScalarParameterValue` "/Game/MyContent/GlobalMaterials/PlayerMaterials/MPC_PlayerAppearance.MPC_PlayerAppearance" "Appearence" _alpha))
    (:`Finished`
      (`self.EnableInput` (`GameplayStatics.GetPlayerController` 0))
      (set `self.IsDead?` false))))

(event `/Game/MyContent/Player/Settings/BI_PlayerControls.MoveRight/Left`
  (params (Axis :type "Float (double-precision)"))
  (bind (_returnvalue_roll _returnvalue_pitch _returnvalue_yaw) (`KismetMathLibrary.BreakRotator` (`self.GetControlRotation`)))
  ;[0.2652 1 0.2584] Movement
  (`self.AddMovementInput` (`KismetMathLibrary.GetRightVector` (`KismetMathLibrary.MakeRotator` 0.0 0.0 _returnvalue_yaw)) Axis))

(event `/Game/MyContent/Player/Settings/BI_PlayerControls.FreeLookPressed`
  ;[0.175 0.2754 1] Free Look
  (set `self.IsFreeLooking?` true))

(event `/Game/MyContent/Player/Settings/BI_PlayerControls.FreeLookReleased`
  ;[1 0.5918 0.07549] Free Look / Need to return to the current character rotation
  (set `self.IsFreeLooking?` false))

(event `/Game/MyContent/Player/Settings/BI_PlayerInteractions.KillPlayer`
  ;[1 1 1] Player Death
  (message `/Game/MyContent/Core/BI_GameInstance.AddDeath` (`GameplayStatics.GetGameInstance`))
  (if (not (`self.IsDead?`)) :!label _label
    (set `self.IsDead?` true)
    (`self.DisableInput` (`GameplayStatics.GetPlayerController` 0))
    ;;[1 0.5918 0.07549] Death Sound
    (`GameplayStatics.PlaySound2D` "/Game/MyContent/Player/Sounds/boom.boom" 1.0 1.0 0.0 null null)
    (bind (_direction _alpha) (`Timeline|Timeline_0` :!via `ReverseFromEnd`)
      (:`Update`
        (`MeshComponent.SetScalarParameterValueOnMaterials` (`self.Mesh`) "Appearence" _alpha)
        (`KismetMaterialLibrary.SetScalarParameterValue` "/Game/MyContent/GlobalMaterials/PlayerMaterials/MPC_PlayerAppearance.MPC_PlayerAppearance" "Appearence" _alpha))
      (:`Finished`
        (`self.Respawn`)))))

(event `/Game/MyContent/Player/Settings/BI_PlayerControls.LookUp/Down`
  (params (Axis :type "Float (double-precision)"))
  ;[0.2652 1 0.2584] Camera Turning
  (`self.AddControllerPitchInput` Axis))

(event `/Game/MyContent/Player/Settings/BI_PlayerControls.FlipFlopCharacterPoV`
  (bind _charactermovement (`self.CharacterMovement`))
  ;[0.175 0.2754 1] FlipFlop Character PoV
  (`/Engine/EditorBlueprintResources/StandardMacros.FlipFlop`
    (:`A`
      (set `CharacterMovementComponent.bOrientRotationToMovement` false _charactermovement)
      (set `CharacterMovementComponent.bUseControllerDesiredRotation` true _charactermovement))
    (:`B`
      (set `CharacterMovementComponent.bOrientRotationToMovement` true _charactermovement)
      (set `CharacterMovementComponent.bUseControllerDesiredRotation` false _charactermovement))))

(event `/Game/MyContent/Player/Settings/BI_PlayerControls.ResetToCheckpoint`
  ;[1 1 1] Player Death
  (message `/Game/MyContent/Core/BI_GameInstance.AddReset` (`GameplayStatics.GetGameInstance`))
  (goto _label))

(event `/Game/MyContent/Player/Settings/BI_PlayerControls.TurnRight/Left`
  (params (`Axis ` :type "Float (double-precision)"))
  ;[0.2652 1 0.2584] Camera Turning
  (bind _output_get (set `self.TurnRate` `Axis `))
  (`self.AddControllerYawInput` _output_get))

(event `/Game/MyContent/Player/Settings/BI_PlayerControls.JumpPressed`
  (bind _charactermovement (`self.CharacterMovement`))
  ;[0.2652 1 0.2584] Jump & Double Jump
  (if (not (`self.IsDashing?`))
    (if (`NavMovementComponent.IsFalling` (`self.CharacterMovement`))
      (bind (_calculated _isavailable_) (`self.CheckFigure` (`self.IsDoubleJumping?`) (`self.CurrentStamina`) (`self.MaxStamina`) (`self.DoubleJumpCost`)))
      (if _isavailable_
        (set `self.CurrentStamina` _calculated)
        (`CharacterMovementComponent.SetMovementMode` _charactermovement "MOVE_Walking" 0)
        (set `self.IsDoubleJumping?` true)
        (set `CharacterMovementComponent.JumpZVelocity` (`self.DoubleJumpZVelocity`) _charactermovement)
        (`self.Jump`)
        (`|PlayMontage` (`self.Mesh`) (`self.DoubleJump`)))
      (else
        (set `self.IsDoubleJumping?` false)
        (set `self.IsJumping?` true)
        (set `CharacterMovementComponent.JumpZVelocity` (`self.JumpZVelocity`) _charactermovement)
        (`self.Jump`)
        (set `self.IsJumping?` false)))))

(event `/Game/MyContent/Player/Settings/BI_PlayerControls.JumpReleased`
  ;[0.2652 1 0.2584] Jump & Double Jump
  (`self.StopJumping`))

(event `/Game/MyContent/Player/Settings/BI_PlayerControls.Crouch/SlidePressed`
  (bind _charactermovement (`self.CharacterMovement`))
  ;[0.2652 1 0.2584] Crouch
  (if (not (`NavMovementComponent.IsFalling` _charactermovement))
    (if (> (`KismetMathLibrary.VSize` (`MovementComponent.Velocity` _charactermovement)) (`self.SlidingLowerLimitSpeed`))
      (`/Engine/EditorBlueprintResources/StandardMacros.DoOnce` false :!label _label_2
        (:`Completed`
          ;[0.175 0.2754 1] Sound
          (`GameplayStatics.PlaySoundAtLocation` "/Game/MyContent/Player/Sounds/Slide/Slide.Slide" (0.0 0.0 0.0) (struct) 2.0 1.0 0.0 null null null null)
          ;[0.175 0.2754 1] Sliding
          (set `CharacterMovementComponent.MaxWalkSpeedCrouched` (`self.RunSpeed`) (`self.CharacterMovement`))
          (`self.Crouch`)
          (`|PlayMontage` (`self.Mesh`) (`self.Sliding`)
            (:`OnCompleted`
              _)
            (:`OnInterrupted`
              _))
          (set `CharacterMovementComponent.MaxWalkSpeedCrouched` (`self.CrouchSpeed`) (`self.CharacterMovement`))
          (goto _label_2 :!via `Reset`))))))

(event `/Game/MyContent/Player/Settings/BI_PlayerControls.Crouch/SlideReleased`
  ;[0.2652 1 0.2584] Crouch
  (`self.UnCrouch` :!label _label_3))

(event `/Game/MyContent/Player/Settings/BI_PlayerControls.CrouchWalk`
  ;[0.2652 1 0.2584] Crouch
  (`/Engine/EditorBlueprintResources/StandardMacros.FlipFlop`
    (:`A`
      (`self.Crouch`))
    (:`B`
      (goto _label_3))))

(event `/Game/MyContent/Player/Settings/BI_PlayerControls.DashSprint`
  (bind _dashmat_ref (`self.DashMat Ref`))
  (bind _charactermovement (`self.CharacterMovement`))
  (bind _returnvalue (* (`KismetMathLibrary.GetForwardVector` (`self.K2_GetActorRotation`)) (`self.DashSpeed`)))
  ;[0.2652 1 0.2584] Dash
  (if (and (`self.CanDash?`) (not (`NavMovementComponent.IsCrouching` (`self.CharacterMovement`))))
    (`/Engine/EditorBlueprintResources/StandardMacros.DoOnce` false :!label _label_4
      (:`Completed`
        (set `self.CanDash?` false)
        (set `self.IsDashing?` true)
        ;;[0.175 0.2754 1] Sound
        (`GameplayStatics.PlaySoundAtLocation` "/Game/MyContent/Player/Sounds/Dash/Dash.Dash" (0.0 0.0 0.0) (struct) 2.0 1.0 0.0 null null null null)
        ;;[0.175 0.2754 1] Dash Motion #1
        (`MaterialInstanceDynamic.SetVectorParameterValue` _dashmat_ref "Loc" (`KismetMathLibrary.Conv_VectorToLinearColor` (* (`SceneComponent.GetForwardVector` (`self.CapsuleComponent`)) -1.0)))
        (`MaterialInstanceDynamic.SetScalarParameterValue` _dashmat_ref "Amount" 0.5)
        (if (not (`NavMovementComponent.IsFalling` (`self.CharacterMovement`)))
          (set `CharacterMovementComponent.GravityScale` 0.0 (`self.CharacterMovement`))
          (`self.LaunchCharacter` _returnvalue)
          (`KismetSystemLibrary.Delay` (`self.DashEffectDuration`))
          (set `self.IsDashing?` false)
          (set `CharacterMovementComponent.GravityScale` 1.0 (`self.CharacterMovement`))
          (else
            (`self.LaunchCharacter` _returnvalue)
            (`KismetSystemLibrary.Delay` (`self.DashEffectDuration`))
            (set `self.IsDashing?` false)
            (set `CharacterMovementComponent.FallingLateralFriction` 5.0 _charactermovement)
            (`KismetSystemLibrary.Delay` 0.1)
            (set `CharacterMovementComponent.FallingLateralFriction` 0.0 _charactermovement)))
        (`MaterialInstanceDynamic.SetScalarParameterValue` (`self.DashMat Ref`) "Amount" 0.0)
        (`KismetSystemLibrary.Delay` (`self.DashCooltime`))
        (set `self.CanDash?` true)
        (goto _label_4 :!via `Reset`)))))

(event `Key|One`
  (params (Key :type "Key Structure"))
  ;[0 0 0] DEBUG
  (:`Pressed`
    (`self.K2_SetActorLocation` (`|GetArrayItem` (`self.Locations`)))))

(event `Key|Seven`
  (params (Key :type "Key Structure"))
  ;[0 0 0] DEBUG
  (:`Pressed`
    (`self.K2_SetActorLocation` (`|GetArrayItem` (`self.Locations`) 6))))

(event `Key|Two`
  (params (Key :type "Key Structure"))
  ;[0 0 0] DEBUG
  (:`Pressed`
    (`self.K2_SetActorLocation` (`|GetArrayItem` (`self.Locations`) 1))))

(event `Key|Three`
  (params (Key :type "Key Structure"))
  ;[0 0 0] DEBUG
  (:`Pressed`
    (`self.K2_SetActorLocation` (`|GetArrayItem` (`self.Locations`) 2))))

(event `Key|Six`
  (params (Key :type "Key Structure"))
  ;[0 0 0] DEBUG
  (:`Pressed`
    (`self.K2_SetActorLocation` (`|GetArrayItem` (`self.Locations`) 5))))

(event `/Game/MyContent/Player/Settings/BI_PlayerInteractions.AddTimerUI`
  ;[1 1 1] Add Timer to UI
  (`/Game/MyContent/Widgets/UI_HUD.EnableTimeUI` (`self.PlayerHud`))
  (set `self.AddTimer?` true))

(event `Key|Four`
  (params (Key :type "Key Structure"))
  ;[0 0 0] DEBUG
  (:`Pressed`
    (`self.K2_SetActorLocation` (`|GetArrayItem` (`self.Locations`) 3))))

(event `/Game/MyContent/Player/Settings/BI_PlayerControls.PauseToggle`
  (bind _returnvalue (`GameplayStatics.GetPlayerController` 0))
  ;[1 1 1] Pause
  (`/Engine/EditorBlueprintResources/StandardMacros.FlipFlop` :!label _label_5
    (:`A`
      (`GameplayStatics.SetGamePaused` true)
      (`Widget.RemoveFromParent` (`self.PlayerHud`))
      (bind _returnvalue_2 (`|CreateWidget` "/Game/MyContent/Maps/MainMenu/UI_PauseMenu.UI_PauseMenu_C" (`GameplayStatics.GetPlayerController` 0)))
      (bind _output_get (set `self.PauseUI` _returnvalue_2))
      (`UserWidget.AddToViewport` _output_get 0))
    (:`B`
      (`GameplayStatics.SetGamePaused` false)
      (bind _foundwidgets (`WidgetBlueprintLibrary.GetAllWidgetsOfClass` "/Game/MyContent/Maps/MainMenu/UI_OptionsMenu.UI_OptionsMenu_C"))
      (for _array_element _foundwidgets
        (`Widget.RemoveFromParent` _array_element)
        (`Widget.RemoveFromParent` (`self.PauseUI`) :!label _label_6)
        (`self.SetUI`)
        (`WidgetBlueprintLibrary.SetInputMode_GameOnly` _returnvalue)
        (set `PlayerController.bShowMouseCursor` false _returnvalue))
      (goto _label_6))))

(event `Key|Five`
  (params (Key :type "Key Structure"))
  ;[0 0 0] DEBUG
  (:`Pressed`
    (`self.K2_SetActorLocation` (`|GetArrayItem` (`self.Locations`) 4))))

(event `Key|Zero` :paused true
  (params (Key :type "Key Structure"))
  ;[1 1 1] Pause
  ;;[0.9316 0 1] Pause for Debug
  (:`Pressed`
    (goto _label_5)))

(event `/Game/MyContent/Player/Settings/BI_PlayerInteractions.SetCheckpointDebug`
  (params (Locations :type "Array of Vector Structure (by ref)"))
  ;[0 0 0] DEBUG
  (set `self.Locations` Locations))

(fn `CheckFigure`
  (params (`IsDoing?` :type Boolean) (CurrentFigure :type "Float (double-precision)") (MaxFigure :type "Float (double-precision)") (Cost :type "Float (double-precision)"))
  (returns (Calculated :type "Float (double-precision)") (`IsAvailable?` :type Boolean))
  (if (and (not `IsDoing?`) (>= CurrentFigure Cost))
    (return (`KismetMathLibrary.FClamp` (- CurrentFigure Cost) 0.0 MaxFigure) true)
    (else
      (return CurrentFigure false))))

(fn `RegenStamina`
  (if (< (`self.CurrentStamina`) (`self.MaxStamina`))
    (set `self.CurrentStamina` (`KismetMathLibrary.FClamp` (+ (`self.CurrentStamina`) (`self.StaminaRegenAmount`)) 0.0 (`self.MaxStamina`)))
    (return)
    (else
      (return))))

(fn `SetUI`
  ;[0.175 0.2754 1] Widget - HUD
  (bind _returnvalue (`|CreateWidget` "/Game/MyContent/Widgets/UI_HUD.UI_HUD_C" null self))
  (bind _output_get (set `self.PlayerHud` _returnvalue))
  (`UserWidget.AddToViewport` _output_get 0))

(fn `UserConstructionScript`)