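; Base player character with camera-relative movement, crouch, double jump, dash and respawn at a stored checkpoint transform.
; A looping timer regenerates stamina, and CheckFigure gates and deducts the cost of double jump and dash.
; Double jump forces Walking mode to jump again with its own Z velocity.
; Ground dash uses a timeline for forward input, animation and speed lines, while air dash only spends stamina and prints.
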(event `self.ReceiveBeginPlay`
  (bind _charactermovement (`self.CharacterMovement`))
  ;[0.175 0.2754 1] Set Movement DefaultValues
  (set `CharacterMovementComponent.MaxWalkSpeed` (`self.RunSpeed`) _charactermovement)
  (set `CharacterMovementComponent.MaxWalkSpeedCrouched` (`self.CrouchSpeed`) _charactermovement)
  (set `CharacterMovementComponent.JumpZVelocity` (`self.JumpZVelocity`) _charactermovement)
  (set `CharacterMovementComponent.MaxAcceleration` (`self.Acceleration`) _charactermovement)
  ;[0.175 0.2754 1] Set StaminaRegen
  (`KismetSystemLibrary.K2_SetTimer` null "RegenStamina" (`self.StaminaRegenInterval`) true))

(event `/Game/MyContent/Player/BI_PlayerControls.MoveForward/Backward`
  (params (Axis :type "Float (double-precision)"))
  (bind (_returnvalue_roll _returnvalue_pitch _returnvalue_yaw) (`KismetMathLibrary.BreakRotator` (`self.GetControlRotation`)))
  ;[0.2652 1 0.2584] Movement
  (`self.AddMovementInput` (`KismetMathLibrary.GetForwardVector` (`KismetMathLibrary.MakeRotator` 0.0 0.0 _returnvalue_yaw)) Axis))

(event `/Game/MyContent/Player/BI_PlayerInteractions.SetPlayerRespawnPoint`
  (params (Respawn :type "Transform Structure"))
  ;[1 1 1] Set Respawn Point
  (set `self.SpawnPoint` Respawn))

(event `Respawn`
  (bind (_spawnpoint_location _spawnpoint_rotation) (`KismetMathLibrary.BreakTransform` (`self.SpawnPoint`)))
  ;[1 1 1] Respawn to last Checkpoint once player has died
  ;;[1 1 1] Move player to spawn point
  (`self.K2_SetActorTransform` (`KismetMathLibrary.MakeTransform` _spawnpoint_location _spawnpoint_rotation) false true))

(event `/Game/MyContent/Player/BI_PlayerControls.MoveRight/Left`
  (params (Axis :type "Float (double-precision)"))
  (bind (_returnvalue_roll _returnvalue_pitch _returnvalue_yaw) (`KismetMathLibrary.BreakRotator` (`self.GetControlRotation`)))
  ;[0.2652 1 0.2584] Movement
  (`self.AddMovementInput` (`KismetMathLibrary.GetRightVector` (`KismetMathLibrary.MakeRotator` _returnvalue_roll 0.0 _returnvalue_yaw)) Axis))

(event `/Game/MyContent/Player/BI_PlayerControls.LookUp/Down`
  (params (Axis :type "Float (double-precision)"))
  ;[0.2652 1 0.2584] Camera Turning
  (`self.AddControllerPitchInput` Axis))

(event `/Game/MyContent/Player/BI_PlayerControls.TurnRight/Left`
  (params (`Axis ` :type "Float (double-precision)"))
  ;[0.2652 1 0.2584] Camera Turning
  (`self.AddControllerYawInput` `Axis `))

(event `/Game/MyContent/Player/BI_PlayerControls.JumpPressed`
  (bind _charactermovement (`self.CharacterMovement`))
  ;[0.2652 1 0.2584] Jump & Double Jump
  (if (`NavMovementComponent.IsFalling` (`self.CharacterMovement`))
    (bind (_calculated _isavailable_) (`self.CheckFigure` (`self.IsDoubleJumping?`) (`self.CurrentStamina`) (`self.MaxStamina`) (`self.DoubleJumpCost`)))
    (if _isavailable_
      (set `self.CurrentStamina` _calculated)
      (`CharacterMovementComponent.SetMovementMode` _charactermovement "MOVE_Walking" 0)
      (set `self.IsDoubleJumping?` true)
      (set `CharacterMovementComponent.JumpZVelocity` (`self.DoubleJumpZVelocity`) _charactermovement)
      (`self.Jump` :!label _label))
    (else
      (set `self.IsDoubleJumping?` false)
      (set `CharacterMovementComponent.JumpZVelocity` (`self.JumpZVelocity`) _charactermovement)
      (goto _label))))

(event `/Game/MyContent/Player/BI_PlayerControls.JumpReleased`
  ;[0.2652 1 0.2584] Jump & Double Jump
  (`self.StopJumping`))

(event `/Game/MyContent/Player/BI_PlayerControls.Crouch/SlidePressed`
  ;[0.2652 1 0.2584] Crouch
  (if (not (`NavMovementComponent.IsFalling` (`self.CharacterMovement`)))
    (`self.Crouch` :!label _label_2)))

(event `/Game/MyContent/Player/BI_PlayerControls.Crouch/SlideReleased`
  ;[0.2652 1 0.2584] Crouch
  (`self.UnCrouch` :!label _label_3))

(event `/Game/MyContent/Player/BI_PlayerControls.CrouchWalk`
  ;[0.2652 1 0.2584] Crouch
  (if (not (`NavMovementComponent.IsFalling` (`self.CharacterMovement`)))
    (`/Engine/EditorBlueprintResources/StandardMacros.FlipFlop`
      (:`A`
        (goto _label_2))
      (:`B`
        (goto _label_3)))))

(event `/Game/MyContent/Player/BI_PlayerControls.DashSprint`
  (bind _mesh (`self.Mesh`))
  (bind _dashlines (`self.DashLines`))
  ;[0.2652 1 0.2584] Dash
  (bind (_calculated _isavailable_) (`self.CheckFigure` (`self.IsDashing?`) (`self.CurrentStamina`) (`self.MaxStamina`) (`self.DashCost`)))
  (if _isavailable_
    (set `self.CurrentStamina` _calculated)
    (set `self.IsDashing?` true)
    (if (not (`NavMovementComponent.IsFalling` (`self.CharacterMovement`)))
      (set `CharacterMovementComponent.MaxWalkSpeed` (`self.DashSpeed`) (`self.CharacterMovement`))
      (`Timeline|Dash` :!via `PlayFromStart`
        (:`Update`
          (`self.AddMovementInput` (`SceneComponent.GetForwardVector` (`self.CapsuleComponent`)))
          (`SkeletalMeshComponent.PlayAnimation` _mesh "/Game/MyContent/Player/Animations/UE5/Locomotion/Customised/UE5_Upperbody_Sprint_Fwd_Montage.UE5_Upperbody_Sprint_Fwd_Montage" false)
          (`ActorComponent.Activate` _dashlines false)
          (`KismetSystemLibrary.Delay` 1.0))
        (:`Finished`
          (set `CharacterMovementComponent.MaxWalkSpeed` (`self.RunSpeed`) (`self.CharacterMovement`))
          (`SkeletalMeshComponent.SetAnimationMode` _mesh "AnimationBlueprint")
          (`ActorComponent.Deactivate` _dashlines)
          (set `self.IsDashing?` false)))
      (else
        (`KismetSystemLibrary.PrintString` "Flying Dash!")
        (`KismetSystemLibrary.Delay` 1.0)
        (set `self.IsDashing?` false)))))

(fn `CheckFigure`
  (params (`IsDoing?` :type Boolean) (CurrentFigure :type "Float (double-precision)") (MaxFigure :type "Float (double-precision)") (Cost :type "Float (double-precision)"))
  (returns (Calculated :type "Float (double-precision)") (`IsAvailable?` :type Boolean))
  (if (and (not `IsDoing?`) (>= CurrentFigure Cost))
    (return (`KismetMathLibrary.FClamp` (- CurrentFigure Cost) 0.0 MaxFigure) true)
    (else
      (return CurrentFigure false))))

(fn `RegenStamina`
  (if (< (`self.CurrentStamina`) (`self.MaxStamina`))
    (bind _output_get (set `self.CurrentStamina` (`KismetMathLibrary.FClamp` (+ (`self.CurrentStamina`) (`self.StaminaRegenAmount`)) 0.0 (`self.MaxStamina`))))
    (`KismetSystemLibrary.PrintString` (`KismetStringLibrary.Concat_StrStr` "My stamina: " (`KismetStringLibrary.Conv_DoubleToString` _output_get)))
    (return)
    (else
      (return))))

(fn `UserConstructionScript`)