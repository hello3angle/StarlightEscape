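; Game mode blueprint that sets game-only input on Begin Play and holds scaffolding for a player stopwatch.
; The Time function adds one second to the PlayersTime timespan and is meant to run on a looping one-second timer.
; Logic to start, stop, pause and adjust that timer exists but is disconnected from its events, so those events currently do nothing.
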(event `self.ReceiveBeginPlay`
  ;[1 1 1] Begin Play
  (`WidgetBlueprintLibrary.SetInputMode_GameOnly` (`GameplayStatics.GetPlayerController` 0)))

(event `AddTime_1`
  (params (Seconds :type Integer))
  ;[1 1 1] Add/Subtract Time
)

(event `TogglePauseTimer_1`
  ;[1 1 1] Pause
)

(event `StopTimer_1`
  ;[1 1 1] Timer
)

(event `SubtractTime_1`
  (params (Seconds :type Integer))
  ;[1 1 1] Add/Subtract Time
)

(event `StartTimer_1`
  ;[1 1 1] Timer
)

(fn `Time`
  (set `self.PlayersTime` (+ (`self.PlayersTime`) (`KismetMathLibrary.MakeTimespan` 0 0 0 1)))
  (return))

(fn `UserConstructionScript`)