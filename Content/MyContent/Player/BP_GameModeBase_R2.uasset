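; BP_GameModeBase_R2 is a game mode that creates the BP_FloorGenerator actor when play begins.
; BeginPlay runs the parent logic, then calls CreateActorGenerator.
; That function destroys any valid existing generator, spawns a new one and stores it in ActorGeneratorRef, so repeated calls replace the tracked instance.
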(event `self.ReceiveBeginPlay`
  (`parent.ReceiveBeginPlay`)
  (`self.CreateActorGenerator`))

(fn `CreateActorGenerator`
  (bind _actorgeneratorref (`self.ActorGeneratorRef`))
  (`/Engine/EditorBlueprintResources/StandardMacros.IsValid` _actorgeneratorref
    (:`Is Valid`
      (`self.K2_DestroyActor` _actorgeneratorref))
    (:`Is Not Valid`
      _))
  (bind _returnvalue (`|SpawnActorFromClass` "/Game/MyContent/Modules/BP_FloorGenerator.BP_FloorGenerator_C" (`KismetMathLibrary.MakeTransform` (0.0 0.0 0.0)) "Undefined" "OverrideRootScale" null null))
  (set `self.ActorGeneratorRef` _returnvalue)
  (return))

(fn `UserConstructionScript`
  (`parent.UserConstructionScript`))