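; Wraith player character, a BP_PlayerBase child with hidden weapon bones that adds slide, crouch and dash moves.
; Crouch input on the ground slides above a speed threshold, raising crouched speed until the montage ends, or crouches otherwise.
; CrouchWalk toggles crouching.
; Dash launches the character forward with boost effects, suspending gravity when grounded, then briefly raises falling lateral friction to brake before a cooldown re-arms it.
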(event `/Game/MyContent/Player/Settings/BI_PlayerControls.Crouch/SlidePressed`
  (bind _charactermovement (`self.CharacterMovement`))
  ;[0.2652 1 0.2584] Crouch
  (if (not (`NavMovementComponent.IsFalling` _charactermovement))
    (if (> (`KismetMathLibrary.VSize` (`MovementComponent.Velocity` _charactermovement)) (`self.SlidingLowerLimitSpeed`))
      (`/Engine/EditorBlueprintResources/StandardMacros.DoOnce` false :!label _label
        (:`Completed`
          (set `self.IsSliding` true)
          ;[0.175 0.2754 1] Sound
          (`GameplayStatics.PlaySoundAtLocation` "/Game/MyContent/Player/Sounds/Slide/Slide.Slide" (0.0 0.0 0.0) (struct) 2.0 1.0 0.0 null null null null)
          ;[0.175 0.2754 1] Sliding
          (set `CharacterMovementComponent.MaxWalkSpeedCrouched` (`self.RunSpeed`) (`self.CharacterMovement`))
          (`self.Crouch`)
          (`|PlayMontage` (`self.Mesh`) (`self.Sliding`)
            (:`OnCompleted`
              _)
            (:`OnInterrupted`
              _))
          (set `self.IsSliding` false)
          (`self.UnCrouch`)
          (set `CharacterMovementComponent.MaxWalkSpeedCrouched` (`self.CrouchSpeed`) (`self.CharacterMovement`))
          (goto _label :!via `Reset`)))
      (else
        (`self.Crouch` :!label _label_2)))))

(event `/Game/MyContent/Player/Settings/BI_PlayerControls.Crouch/SlideReleased`
  ;[0.2652 1 0.2584] Crouch
  (if (< (`CharacterMovementComponent.MaxWalkSpeedCrouched` (`self.CharacterMovement`)) (`self.RunSpeed`))
    (`self.UnCrouch` :!label _label_3)))

(event `/Game/MyContent/Player/Settings/BI_PlayerControls.CrouchWalk`
  ;[0.2652 1 0.2584] Crouch
  (`/Engine/EditorBlueprintResources/StandardMacros.FlipFlop`
    (:`A`
      (goto _label_2))
    (:`B`
      (goto _label_3))))

(event `/Game/MyContent/Player/Settings/BI_PlayerControls.DashSprint`
  (bind _charactermovement (`self.CharacterMovement`))
  (bind _returnvalue (* (`KismetMathLibrary.GetForwardVector` (`self.K2_GetActorRotation`)) (`self.DashSpeed`)))
  ;[0.2652 1 0.2584] Dash
  (if (and (`self.CanDash?`) (not (`NavMovementComponent.IsCrouching` (`self.CharacterMovement`))))
    (`/Engine/EditorBlueprintResources/StandardMacros.DoOnce` false :!label _label_4
      (:`Completed`
        (set `self.CanDash?` false)
        (set `self.IsDashing?` true)
        ;;[0.175 0.2754 1] Sound
        (`GameplayStatics.PlaySoundAtLocation` "/Game/MyContent/Player/Sounds/Dash/Dash.Dash" (0.0 0.0 0.0) (struct) 2.0 1.0 0.0 null null null null)
        ;;[0.175 0.2754 1] Dash Motion #1
        (`ActorComponent.Activate` (`self.Boost_R`) true)
        (`ActorComponent.Activate` (`self.Boost_L`) true)
        (if (not (`NavMovementComponent.IsFalling` (`self.CharacterMovement`)))
          (set `CharacterMovementComponent.GravityScale` 0.0 (`self.CharacterMovement`))
          (`self.LaunchCharacter` _returnvalue)
          (`KismetSystemLibrary.Delay` (`self.DashEffectDuration`))
          (set `CharacterMovementComponent.GravityScale` 1.0 (`self.CharacterMovement`))
          (else
            (`self.LaunchCharacter` _returnvalue)
            (`KismetSystemLibrary.Delay` (`self.DashEffectDuration`))))
        (set `CharacterMovementComponent.FallingLateralFriction` 5.0 _charactermovement)
        (`KismetSystemLibrary.Delay` 0.1)
        (set `CharacterMovementComponent.FallingLateralFriction` 0.0 _charactermovement)
        (set `self.IsDashing?` false)
        (`KismetSystemLibrary.Delay` (`self.DashCooltime`))
        (set `self.CanDash?` true)
        (goto _label_4 :!via `Reset`)))))

(fn `UserConstructionScript`
  (bind _mesh (`self.Mesh`))
  (`parent.UserConstructionScript`)
  (`SkinnedMeshComponent.HideBoneByName` _mesh "weapon_r" "PBO_None")
  (`SkinnedMeshComponent.HideBoneByName` _mesh "weapon_l" "PBO_None"))