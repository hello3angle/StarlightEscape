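; Background music manager that switches the game to a new BGM track through its FadeToNewBGM event.
; It alternates between two audio components, BGMAudio and BGM2, using whether BGMAudio holds a valid sound to choose which receives and fades in the new track.
; A fade-out is called for the outgoing side, whose sound is then cleared immediately, flipping the choice for the next switch.
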(event `FadeToNewBGM`
  (params (NewBGM :type "SoundCue Object Reference"))
  (`/Engine/EditorBlueprintResources/StandardMacros.IsValid` (`AudioComponent.Sound` (`self.BGMAudio`))
    (:`Is Valid`
      (`AudioComponent.SetSound` (`self.BGM2`) NewBGM)
      (`self.FadeOut`)
      (`AudioComponent.FadeIn` (`self.BGM2`) (`self.Fade in Duration`) 1.0 0.0 "Linear")
      (`AudioComponent.SetSound` (`self.BGMAudio`) null))
    (:`Is Not Valid`
      (`AudioComponent.SetSound` (`self.BGMAudio`) NewBGM)
      (`AudioComponent.FadeOut` (`self.BGM2`) (`self.Fade Out Duration`) 0.0 "Linear")
      (`AudioComponent.FadeIn` (`self.BGMAudio`) (`self.Fade in Duration`) 1.0 0.0 "Linear")
      (`AudioComponent.SetSound` (`self.BGM2`) null))))

(fn `UserConstructionScript`
  (`parent.UserConstructionScript`))