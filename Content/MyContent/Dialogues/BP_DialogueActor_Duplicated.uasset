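; BP_DialogueActor_Duplicated is a trigger-box actor that plays a dialogue cutscene, then moves the game to Lvl_Outro.
; Player overlap calls ShowDialogue, which, given a valid LevelSequence, disables input, hides the pawn and plays the sequence.
; A timer set one second before the sequence ends re-enables input, shows a WS_FadeScreen fade-out widget and opens the outro level after a short delay.
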(event `self.ReceiveBeginPlay`)

(event `self.Box.OnComponentBeginOverlap`
  (params (OverlappedComponent :type "PrimitiveComponent Object Reference") (OtherActor :type "Actor Object Reference") (OtherComp :type "PrimitiveComponent Object Reference") (OtherBodyIndex :type Integer) (bFromSweep :type Boolean) (SweepResult :type "HitResult Structure (by ref)"))
  (cast `/Game/MyContent/Player/BP_PlayerBase` OtherActor)
  (`/Game/MyContent/Dialogues/BI_DialogueInteractions.ShowDialogue`))

(event `/Game/MyContent/Dialogues/BI_DialogueInteractions.ShowDialogue`
  (`/Engine/EditorBlueprintResources/StandardMacros.IsValid` (`self.LevelSequence`)
    (:`Is Valid`
      (`self.DisableInput` (`GameplayStatics.GetPlayerController` 0) null)
      (bind (_outactor _returnvalue) (`LevelSequencePlayer.CreateLevelSequencePlayer` (`self.LevelSequence`)))
      (`self.SetActorHiddenInGame` (`GameplayStatics.GetPlayerPawn` 0) true)
      (`MovieSceneSequencePlayer.Play` _returnvalue)
      (`KismetSystemLibrary.K2_SetTimerDelegate` (delegate `EnableInputKeys`) (- (`TimeManagementBlueprintLibrary.Conv_QualifiedFrameTimeToSeconds` (`MovieSceneSequencePlayer.GetDuration` _returnvalue)) 1.0)))))

(event `EnableInputKeys`
  (`self.EnableInput` (`GameplayStatics.GetPlayerController` 0) null)
  (bind _returnvalue (`|CreateWidget` "/Game/MyContent/Widgets/WS_FadeScreen.WS_FadeScreen_C"))
  (`/Game/MyContent/Widgets/WS_FadeScreen.FadeOut` _returnvalue)
  (`UserWidget.AddToViewport` _returnvalue 0)
  (`KismetSystemLibrary.Delay` 1.0)
  (`GameplayStatics.OpenLevel` "Lvl_Outro")
  (`KismetSystemLibrary.Delay` 1.0)
  (`Widget.RemoveFromParent` _returnvalue))

(fn `UserConstructionScript`)