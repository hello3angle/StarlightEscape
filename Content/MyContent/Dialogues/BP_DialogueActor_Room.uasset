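; Trigger-box actor that presents a tutorial moment on overlap while its IsTutorial flag is set.
; Overlap toggles the pause-timer message on the GameInstance and hides the player's HUD.
; A valid level sequence plays with input disabled, then a duration-based timer restores input and HUD, toggles the message again and disables box collision.
; Without a sequence, it shows a dialogue widget with title and text and clears the flag.
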(event `self.ReceiveBeginPlay`)

(event `self.Box.OnComponentBeginOverlap`
  (params (OverlappedComponent :type "PrimitiveComponent Object Reference") (OtherActor :type "Actor Object Reference") (OtherComp :type "PrimitiveComponent Object Reference") (OtherBodyIndex :type Integer) (bFromSweep :type Boolean) (SweepResult :type "HitResult Structure (by ref)"))
  (set `self.player` OtherActor)
  (`/Game/MyContent/Dialogues/BI_DialogueInteractions.ShowDialogue`)
  (message `/Game/MyContent/Core/BI_GameInstance.TogglePauseTimer` (`GameplayStatics.GetGameInstance`))
  (message `/Game/MyContent/Player/Settings/BI_PlayerInteractions.HidePlayerHUD` (`self.player`)))

(event `/Game/MyContent/Dialogues/BI_DialogueInteractions.ShowDialogue`
  (if (`self.IsTutorial?`)
    (`/Engine/EditorBlueprintResources/StandardMacros.IsValid` (`self.LevelSequence`)
      (:`Is Valid`
        (`self.DisableInput` (`GameplayStatics.GetPlayerController` 0) null)
        (bind (_outactor _returnvalue) (`LevelSequencePlayer.CreateLevelSequencePlayer` (`self.LevelSequence`)))
        (`MovieSceneSequencePlayer.Play` _returnvalue)
        (`KismetSystemLibrary.K2_SetTimerDelegate` (delegate `EnableInputKeys`) (`TimeManagementBlueprintLibrary.Conv_QualifiedFrameTimeToSeconds` (`MovieSceneSequencePlayer.GetDuration` _returnvalue))))
      (:`Is Not Valid`
        (bind _returnvalue_2 (`|CreateWidget` "/Game/MyContent/Dialogues/WSUI_Dialogue.WSUI_Dialogue_C"))
        (bind _output_get (set `self.DialogueUI` _returnvalue_2))
        (set `/Game/MyContent/Dialogues/WSUI_Dialogue.TitleText` (`self.TitleText`) _output_get)
        (set `/Game/MyContent/Dialogues/WSUI_Dialogue.DialogueText` (`self.DialogueText`) _output_get)
        (`UserWidget.AddToViewport` (`self.DialogueUI`) 0)
        (set `self.IsTutorial?` false)))))

(event `self.Box.OnComponentEndOverlap`
  (params (OverlappedComponent :type "PrimitiveComponent Object Reference") (OtherActor :type "Actor Object Reference") (OtherComp :type "PrimitiveComponent Object Reference") (OtherBodyIndex :type Integer)))

(event `EnableInputKeys`
  (`self.EnableInput` (`GameplayStatics.GetPlayerController` 0) null)
  (set `self.IsTutorial?` false)
  (message `/Game/MyContent/Core/BI_GameInstance.TogglePauseTimer` (`GameplayStatics.GetGameInstance`))
  (message `/Game/MyContent/Player/Settings/BI_PlayerInteractions.ShowPlayerHUD` (`self.player`))
  (`PrimitiveComponent.SetCollisionEnabled` (`self.Box`) "NoCollision"))

(fn `UserConstructionScript`)