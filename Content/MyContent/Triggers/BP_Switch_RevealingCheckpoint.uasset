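; Checkpoint trigger that reveals hidden platforms and actors when its box is overlapped.
; On BeginPlay it messages each entry in PlatformsToReveal to hide and sets each entry in ActorsToReveal hidden in game.
; Box overlap passes the overlapping actor to SetCheckpoint, then sends the platforms a reveal message and unhides the actors, with no actor filter in this graph.
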(event `self.ReceiveBeginPlay`
  (`parent.ReceiveBeginPlay`)
  (for _array_element (`self.PlatformsToReveal`)
    (message `/Game/MyContent/Platforms/BI_Platforms.HidePlatform` _array_element))
  (for _array_element_2 (`self.ActorsToReveal`)
    (`self.SetActorHiddenInGame` _array_element_2 true)))

(event `self.Box.OnComponentBeginOverlap`
  (params (OverlappedComponent :type "PrimitiveComponent Object Reference") (OtherActor :type "Actor Object Reference") (OtherComp :type "PrimitiveComponent Object Reference") (OtherBodyIndex :type Integer) (bFromSweep :type Boolean) (SweepResult :type "HitResult Structure (by ref)"))
  (`self.SetCheckpoint` OtherActor)
  (for _array_element (`self.PlatformsToReveal`)
    (message `/Game/MyContent/Platforms/BI_Platforms.RevealPlatform` _array_element))
  (for _array_element_2 (`self.ActorsToReveal`)
    (`self.SetActorHiddenInGame` _array_element_2 false)))

(fn `UserConstructionScript`
  (`parent.UserConstructionScript`))