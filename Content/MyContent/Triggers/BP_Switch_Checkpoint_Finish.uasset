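; Finish-line variant of a checkpoint switch trigger that ends the level.
; When an actor overlaps its box, it sets the checkpoint for that actor and pauses the timer on BP_GameModeBase.
; It then disables box collision, raises the Emissive parameter on two materials to light up, and opens the MainMenu level.
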(event `self.Box.OnComponentBeginOverlap`
  (params (OverlappedComponent :type "PrimitiveComponent Object Reference") (OtherActor :type "Actor Object Reference") (OtherComp :type "PrimitiveComponent Object Reference") (OtherBodyIndex :type Integer) (bFromSweep :type Boolean) (SweepResult :type "HitResult Structure (by ref)"))
  (`self.SetCheckpoint` OtherActor)
  (bind _asbp_game_mode_base (cast `/Game/MyContent/Player/BP_GameModeBase` (`GameplayStatics.GetGameMode`)))
  (`/Game/MyContent/Player/BP_GameModeBase.PauseTimer` _asbp_game_mode_base)
  (`PrimitiveComponent.SetCollisionEnabled` (`self.Box`) "NoCollision")
  (`MaterialInstanceDynamic.SetScalarParameterValue` (`self.Material1`) "Emissive" 50.0)
  (`MaterialInstanceDynamic.SetScalarParameterValue` (`self.Material2`) "Emissive" 50.0)
  (`GameplayStatics.OpenLevelBySoftObjectPtr` "/Game/MyContent/MainMenu/MainMenu.MainMenu"))

(fn `UserConstructionScript`
  (`parent.UserConstructionScript`))