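; Motion-triggered downlight that switches on when something overlaps its detection box, with no logic to switch it off again.
; On BeginPlay, a visibility line trace along the Arrow measures the distance to the first hit, which sizes and positions the Box and offsets the SMLamp04 mesh.
; The first overlap shows both point lights, swaps both lamp meshes to a lit material and disables Box collision, making the trigger one-shot.
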(event `self.ReceiveBeginPlay`
  (bind _arrow (`self.Arrow`))
  (bind _box (`self.Box`))
  (bind (_returnvalue_x _returnvalue_y) (`KismetMathLibrary.BreakVector` (`BoxComponent.GetUnscaledBoxExtent` _box)))
  (bind _returnvalue (`SceneComponent.K2_GetComponentLocation` _arrow))
  (bind (_outhit _returnvalue_2) (`KismetSystemLibrary.LineTraceSingle` _returnvalue (+ _returnvalue (* (`SceneComponent.GetForwardVector` _arrow) (`self.LineTraceLength`))) "TraceTypeQuery1"))
  (if _returnvalue_2
    (bind _returnvalue_3 (/ (`.Distance` (`GameplayStatics.BreakHitResult` _outhit)) 6.0))
    (`BoxComponent.SetBoxExtent` _box (`KismetMathLibrary.MakeVector` _returnvalue_x _returnvalue_y _returnvalue_3) true)
    (bind _result (`/Engine/EditorBlueprintResources/StandardMacros.NegateFloat` _returnvalue_3)
      (:`  `
        (`SceneComponent.K2_SetRelativeLocation` (`self.Box`) (`KismetMathLibrary.MakeVector` 0.0 0.0 _result) false false)
        (`SceneComponent.K2_SetRelativeLocation` (`self.SM_Lamp_04`) (`KismetMathLibrary.MakeVector` 0.0 0.0 (+ (* _result 6.0) 10.0)) false false)))))

(event `self.Box.OnComponentBeginOverlap`
  (params (OverlappedComponent :type "PrimitiveComponent Object Reference") (OtherActor :type "Actor Object Reference") (OtherComp :type "PrimitiveComponent Object Reference") (OtherBodyIndex :type Integer) (bFromSweep :type Boolean) (SweepResult :type "HitResult Structure (by ref)"))
  (`SceneComponent.SetVisibility` (`self.PointLight`) true false)
  (`SceneComponent.SetVisibility` (`self.PointLight1`) true false)
  (`PrimitiveComponent.SetCollisionEnabled` (`self.Box`) "NoCollision")
  (`PrimitiveComponent.SetMaterial` (`self.SM_Lamp_03`) 1 "/Game/MyContent/Lights/ModularSciFiOffice/Materials/Lights/MI_Light.MI_Light")
  (`PrimitiveComponent.SetMaterial` (`self.SM_Lamp_04`) 1 "/Game/MyContent/Lights/ModularSciFiOffice/Materials/Lights/MI_Light.MI_Light"))

(fn `UserConstructionScript`
  (`parent.UserConstructionScript`))