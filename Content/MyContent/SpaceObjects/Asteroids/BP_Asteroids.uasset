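; Asteroid ring actor that builds a band of instanced meshes and spins slowly around its local Z axis on Tick.
; The construction script sets the mesh and cull distances on a hierarchical instanced static mesh, then fills a length-by-width grid of instances.
; TransformAsteroid wraps that grid around the ring radius, using a random stream to jitter position and blend ring-aligned rotation toward random.
; Instance scale grows with width index rather than being randomised.
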(event `self.ReceiveTick`
  (params (DeltaSeconds :type "Float (single-precision)"))
  (`self.K2_AddActorLocalRotation` (`KismetMathLibrary.RotatorFromAxisAndAngle` (0.0 0.0 1.0) (* DeltaSeconds (`self.RotationSpeed`)))))

(fn `TransformAsteroid`
  (params (`Index from Width Loop` :type Integer) (`Instancec by Width` :type Integer) (`Index from Length Loop` :type Integer) (`Instances by Length` :type Integer))
  (returns (OutLocation :type "Vector Structure") (OutRotation :type "Rotator Structure"))
  (bind _returnvalue (`KismetMathLibrary.MakeVector` 0.0 0.0 1.0))
  (bind _transformrandom (`self.TransformRandom`))
  (bind _returnvalue_2 (`KismetMathLibrary.RotateAngleAxis` (+ (+ (* (- (`KismetMathLibrary.RandomFloatFromStream` _transformrandom) 0.5) (`self.RandomiseZAxisPosition`) (`self.RingWidth`)) (* (`KismetMathLibrary.RandomUnitVectorFromStream` _transformrandom) (`self.RandomisePosition`))) (`KismetMathLibrary.MakeVector` 0.0 (+ (`self.RingRadius`) (* (- (/ (`KismetMathLibrary.Conv_IntToDouble` `Index from Width Loop`) (`KismetMathLibrary.Conv_IntToDouble` `Instancec by Width`)) 0.5) (`self.RingWidth`))))) (* (/ (`KismetMathLibrary.Conv_IntToDouble` `Index from Length Loop`) (`KismetMathLibrary.Conv_IntToDouble` `Instances by Length`)) 360.0) _returnvalue))
  (return _returnvalue_2 (`KismetMathLibrary.RLerp` (`KismetMathLibrary.MakeRotFromYZ` (`KismetMathLibrary.Cross_VectorVector` _returnvalue _returnvalue_2) _returnvalue) (`KismetMathLibrary.RandomRotatorFromStream` true (`self.TransformRandom`)) (`self.RandomiseRotation`) true)))

(fn `UserConstructionScript`
  (bind _hierarchicalinstancedstaticspawn (`self.HierarchicalInstancedStaticSpawn`))
  (bind _instancecountbylength (`self.InstanceCountByLength`))
  (bind _instancecountbywidth (`self.InstanceCountByWidth`))
  (`|ExecutionSequence`
    (:`then_0`
      (`StaticMeshComponent.SetStaticMesh` _hierarchicalinstancedstaticspawn (`self.InstanceMesh`)))
    (:`then_1`
      (`InstancedStaticMeshComponent.SetCullDistances` _hierarchicalinstancedstaticspawn (`self.CullingNear`) (`self.CullingFar`)))
    (:`then_2`
      (for _index (range _instancecountbylength)
        (for _index_2 (range _instancecountbywidth)
          (bind (_outlocation _outrotation) (`self.TransformAsteroid` _index_2 _instancecountbywidth _index _instancecountbylength))
          (`InstancedStaticMeshComponent.AddInstance` (`self.HierarchicalInstancedStaticSpawn`) (`KismetMathLibrary.MakeTransform` _outlocation _outrotation (`KismetMathLibrary.Conv_DoubleToVector` (* _index_2 (`self.MinimumRandomScale`)))) false))))))