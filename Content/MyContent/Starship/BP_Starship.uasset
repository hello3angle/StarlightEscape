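; BP_Starship is a starship actor with four Niagara-style booster exhaust effects, two on the left and two on the right.
; On BeginPlay it passes its IsOn flag to the BoosterOn/Off function.
; That function activates all four exhaust components when on and deactivates them when off, with no tick or overlap logic.
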(event `self.ReceiveBeginPlay`
  (`self.BoosterOn/Off` (`self.IsOn?`)))

(fn `BoosterOn/Off`
  (params (`IsOn?` :type Boolean))
  (bind _ns_boosterexhaust_r1 (`self.NS_BoosterExhaust_R1`))
  (if `IsOn?`
    (`ActorComponent.Activate` _ns_boosterexhaust_r1 false)
    (`ActorComponent.Activate` (`self.NS_BoosterExhaust_L1`) false)
    (`ActorComponent.Activate` (`self.NS_BoosterExhaust_R2`) false)
    (`ActorComponent.Activate` (`self.NS_BoosterExhaust_L2`) false)
    (else
      (`ActorComponent.Deactivate` _ns_boosterexhaust_r1)
      (`ActorComponent.Deactivate` (`self.NS_BoosterExhaust_L1`))
      (`ActorComponent.Deactivate` (`self.NS_BoosterExhaust_R2`))
      (`ActorComponent.Deactivate` (`self.NS_BoosterExhaust_L2`))))
  (return))

(fn `UserConstructionScript`)