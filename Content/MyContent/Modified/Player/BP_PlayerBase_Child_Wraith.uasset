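; Wraith player character, a child of the player base, whose sprint input performs a cooldown-gated forward dash.
; The dash plays a sound, activates both boost effects, drives a dash material's direction and amount, and launches the character along its facing.
; Grounded dashes suspend gravity for the effect duration, while airborne dashes briefly raise falling lateral friction afterward to brake.
; The construction script hides both weapon bones on the mesh.
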(event `/Game/MyContent/Player/BI_PlayerControls.DashSprint`
  (bind _dashmat_ref (`self.DashMat Ref`))
  (bind _charactermovement (`self.CharacterMovement`))
  (bind _returnvalue (* (`KismetMathLibrary.GetForwardVector` (`self.K2_GetActorRotation`)) (`self.DashSpeed`)))
  ;[0.2652 1 0.2584] Dash
  (if (and (`self.CanDash?`) (not (`NavMovementComponent.IsCrouching` (`self.CharacterMovement`))))
    (`/Engine/EditorBlueprintResources/StandardMacros.DoOnce` false :!label _label
      (:`Completed`
        (set `self.CanDash?` false)
        (set `self.IsDashing?` true)
        ;;[0.175 0.2754 1] Sound
        (`GameplayStatics.PlaySoundAtLocation` "/Game/MyContent/Player/Sounds/Dash/Dash.Dash" (0.0 0.0 0.0) (struct) 2.0 1.0 0.0 null null null null)
        ;;[0.175 0.2754 1] Dash Motion #1
        (`ActorComponent.Activate` (`self.Boost_R`) true)
        (`ActorComponent.Activate` (`self.Boost_L`) true)
        (`MaterialInstanceDynamic.SetVectorParameterValue` _dashmat_ref "Loc" (`KismetMathLibrary.Conv_VectorToLinearColor` (* (`SceneComponent.GetForwardVector` (`self.CapsuleComponent`)) -1.0)))
        (`MaterialInstanceDynamic.SetScalarParameterValue` _dashmat_ref "Amount" 0.5)
        (if (not (`NavMovementComponent.IsFalling` (`self.CharacterMovement`)))
          (set `CharacterMovementComponent.GravityScale` 0.0 (`self.CharacterMovement`))
          (`self.LaunchCharacter` _returnvalue)
          (`KismetSystemLibrary.Delay` (`self.DashEffectDuration`))
          (set `self.IsDashing?` false)
          (set `CharacterMovementComponent.GravityScale` 1.0 (`self.CharacterMovement`))
          (else
            (`self.LaunchCharacter` _returnvalue)
            (`KismetSystemLibrary.Delay` (`self.DashEffectDuration`))
            (set `self.IsDashing?` false)
            (set `CharacterMovementComponent.FallingLateralFriction` 5.0 _charactermovement)
            (`KismetSystemLibrary.Delay` 0.1)
            (set `CharacterMovementComponent.FallingLateralFriction` 0.0 _charactermovement)))
        (`MaterialInstanceDynamic.SetScalarParameterValue` (`self.DashMat Ref`) "Amount" 0.0)
        (`KismetSystemLibrary.Delay` (`self.DashCooltime`))
        (set `self.CanDash?` true)
        (goto _label :!via `Reset`)))))

(fn `UserConstructionScript`
  (bind _mesh (`self.Mesh`))
  (`parent.UserConstructionScript`)
  (`SkinnedMeshComponent.HideBoneByName` _mesh "weapon_r" "PBO_None")
  (`SkinnedMeshComponent.HideBoneByName` _mesh "weapon_l" "PBO_None"))